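; Crowd spawner that populates the Bound volume with SpawnAmount BP_Foule actors on BeginPlay.
; Each SpawnCharacter call traces from high above random points in the bounds along the actor's down vector against WorldStatic objects to find the ground.
; It spawns just above the trace location without checking for a hit, with yaw from RandomFloat (0–1 degree), adjusting or skipping colliding spawns to prevent overlap.
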(event EventBeginPlay
  (for _index (range 1 (Variables|Default|GetSpawn%20Amount))
    (CallFunction|SpawnCharacter)))

(fn ConstructionScript)

(fn SpawnCharacter
  (bind _bound (Variables|Default|GetBound))
  (bind (_origin _boxextent) (Collision|GetComponentBounds _bound))
  (bind _returnvalue (Math|Random|RandomPointinBoundingBox _origin _boxextent))
  (bind (_x _y _z) (Math|Vector|BreakVector _returnvalue))
  (bind _returnvalue_2 (+ _z 1e+04))
  (bind _returnvalue_3 (Math|Vector|MakeVector _x _y _returnvalue_2))
  ;[1 1 1] La fonction permet de faire spawn un nombre défini dans la variable "Spawn Amount" de  bp_Foule qui se cale sur le sol et spawn dans la box de collision. Ils ne peuvent pas se superposer
  (bind _outhit (Collision|LineTraceForObjects _returnvalue_3 (+ _returnvalue_3 (* (* (Transformation|GetActorUpVector) -1) 1.5e+04)) (Utilities|Array|MakeArray "ObjectTypeQuery1") false 0 "None"))
  ;;[1 0.09273 0.2833] Fait apparaitre le bp et empêche la supperosition
  (Game|SpawnActorfromClass "/Game/Environnement/Foule/BP_Foule.BP_Foule_C" (Math|Transform|MakeTransform (Math|Vector|MakeVector (.X (Math|Vector|BreakVector (.Location (Collision|BreakHitResult _outhit)))) (.Y (Math|Vector|BreakVector (.Location (Collision|BreakHitResult _outhit)))) (+ (.Z (Math|Vector|BreakVector (.Location (Collision|BreakHitResult _outhit)))) 1.0)) (Math|Rotator|MakeRotator 0.0 0.0 (Math|Random|RandomFloat))) "AdjustIfPossibleButDontSpawnIfColliding" "MultiplyWithRoot" 0 0))