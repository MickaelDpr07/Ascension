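; Crowd NPC that gets a random body colour and a random behavior tree at BeginPlay, with logic for eating and queueing at food stalls (BP_Echoppe).
; Its events pick a random stall, toggle its occupied flag and write destinations and state to Blackboard keys.
; If the stall is busy, it recursively scans BP_FileAttente child-actor slots to claim a free one, or flags NoPlace.
; When the stall frees up, it releases its slot and targets the previous one.
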(event Custom|Choisir_Echoppe
  ;[1 0.4922 0] Manger
  ;;[0 1 0.6484] Choix de l'échoppe
  (bind _outactors (Actor|GetAllActorsOfClass "/Game/Environnement/Foule/Elements_Interactif/BP_Echoppe/BP_Echoppe.BP_Echoppe_C"))
  (bind _output_get (Variables|Default|SetEchoppeChoisi (Utilities|Array|Get(acopy) _outactors (Math|Random|RandomInteger (Utilities|Array|Length _outactors)))))
  (AI|Components|Blackboard|SetValueasVector (AI|GetBlackboard 0) (Utilities|Name|MakeLiteralName "SpotLocation") (Transformation|GetWorldLocation (Variables|/Game/Environnement/Foule/Elements_Interactif/BP_Echoppe/BP_Echoppe.BP_Echoppe_C|GetTarget _output_get))))

(event Custom|CheckSiQuelqu'unMange
  (bind _returnvalue (AI|GetBlackboard 0))
  (bind _returnvalue_2 (AI|GetBlackboard 0))
  ;[1 0.4922 0] Manger
  ;;[0.8984 1 0] Check si Quelqu'un Mange
  (if (Variables|/Game/Environnement/Foule/Elements_Interactif/BP_Echoppe/BP_Echoppe.BP_Echoppe_C|GetQuelqu'unMange (Variables|Default|GetEchoppeChoisi))
    (AI|Components|Blackboard|SetValueasBool (AI|GetBlackboard 0) (Utilities|Name|MakeLiteralName "Table Libre?") false)
    (AI|Components|Blackboard|SetValueasBool (AI|GetBlackboard 0) (Utilities|Name|MakeLiteralName "GoFile") true)
    (bind _asbp_file_attente (Utilities|Casting|CastToBP_FileAttente (Variables|/Script/Engine.ChildActorComponent|GetChildActor (Utilities|Array|Get(acopy) (Variables|/Game/Environnement/Foule/Elements_Interactif/BP_Echoppe/BP_Echoppe.BP_Echoppe_C|GetFileD'attente (Variables|Default|GetEchoppeChoisi)) (Variables|Default|GetFiled'attente%20à%20tester)))))
    (if (Variables|/Game/Environnement/Foule/Elements_Interactif/BP_Echoppe/BP_FileAttente.BP_FileAttente_C|GetPlacePrise _asbp_file_attente)
      (bind _output_get (Variables|Default|SetFiled'attente%20à%20tester (+ (Variables|Default|GetFiled'attente%20à%20tester) 1)))
      (if (== _output_get (Utilities|Array|Length (Variables|/Game/Environnement/Foule/Elements_Interactif/BP_Echoppe/BP_Echoppe.BP_Echoppe_C|GetFileD'attente (Variables|Default|GetEchoppeChoisi))))
        (AI|Components|Blackboard|SetValueasBool _returnvalue (Utilities|Name|MakeLiteralName "GoFile") false)
        (AI|Components|Blackboard|SetValueasBool _returnvalue (Utilities|Name|MakeLiteralName "IsChecking") false)
        (AI|Components|Blackboard|SetValueasBool _returnvalue (Utilities|Name|MakeLiteralName "NoPlace") true)
        (Variables|Default|SetFiled'attente%20à%20tester 0)
        (else
          (CallFunction|CheckSiQuelqu'unMange)))
      (else
        (CallFunction|FileD'attente _asbp_file_attente)))
    (else
      (AI|Components|Blackboard|SetValueasBool (AI|GetBlackboard 0) (Utilities|Name|MakeLiteralName "Table Libre?") true)
      (AI|Components|Blackboard|SetValueasVector (AI|GetBlackboard 0) (Utilities|Name|MakeLiteralName "SpotLocation") (Transformation|GetWorldLocation (Variables|/Game/Environnement/Foule/Elements_Interactif/BP_Echoppe/BP_Echoppe.BP_Echoppe_C|GetTarget (Variables|Default|GetEchoppeChoisi))))
      (AI|Components|Blackboard|SetValueasBool _returnvalue_2 (Utilities|Name|MakeLiteralName "NoPlace") false)
      (AI|Components|Blackboard|SetValueasBool _returnvalue_2 (Utilities|Name|MakeLiteralName "GoFile") false))))

(event Custom|Mange
  ;[1 0.4922 0] Manger
  ;;[1 0 0.1641] Manger
  (Variables|/Game/Environnement/Foule/Elements_Interactif/BP_Echoppe/BP_Echoppe.BP_Echoppe_C|SetQuelqu'unMange (Variables|Default|GetEchoppeChoisi) true))

(event Custom|Liberez%20Place%20File
  ;[1 0.4922 0] Manger
  ;;[0.6406 0 1] Libération Place File d'attente
  (if (Variables|/Game/Environnement/Foule/Elements_Interactif/BP_Echoppe/BP_Echoppe.BP_Echoppe_C|GetQuelqu'unMange (Variables|Default|GetEchoppeChoisi))
    (AI|Components|Blackboard|SetValueasBool (AI|GetBlackboard 0) (Utilities|Name|MakeLiteralName "GoFile") true)
    (else
      (bind _asbp_file_attente (Utilities|Casting|CastToBP_FileAttente (Variables|/Script/Engine.ChildActorComponent|GetChildActor (Utilities|Array|Get(acopy) (Variables|/Game/Environnement/Foule/Elements_Interactif/BP_Echoppe/BP_Echoppe.BP_Echoppe_C|GetFileD'attente (Variables|Default|GetEchoppeChoisi)) (Variables|Default|GetFiled'attente%20à%20tester)))))
      (Variables|/Game/Environnement/Foule/Elements_Interactif/BP_Echoppe/BP_FileAttente.BP_FileAttente_C|SetPlacePrise _asbp_file_attente false)
      (CallFunction|LiébrationPlaceFile _asbp_file_attente))))

(event Custom|Fini%20Manger
  (bind _returnvalue (AI|GetBlackboard 0))
  ;[1 0.4922 0] Manger
  ;;[0.3594 0 1] Fini Manger
  (Variables|/Game/Environnement/Foule/Elements_Interactif/BP_Echoppe/BP_Echoppe.BP_Echoppe_C|SetQuelqu'unMange (Variables|Default|GetEchoppeChoisi) false)
  (AI|Components|Blackboard|SetValueasBool _returnvalue (Utilities|Name|MakeLiteralName "IsChecking") false)
  (AI|Components|Blackboard|SetValueasBool _returnvalue (Utilities|Name|MakeLiteralName "GoFile") false))

(event Custom|Check%20if%20table%20libre
  (bind _returnvalue (Utilities|Name|MakeLiteralName "Table Libre?"))
  (bind _returnvalue_2 (AI|GetBlackboard 0))
  ;[1 0.4922 0] Manger
  (if (Variables|/Game/Environnement/Foule/Elements_Interactif/BP_Echoppe/BP_Echoppe.BP_Echoppe_C|GetQuelqu'unMange (Variables|Default|GetEchoppeChoisi))
    (AI|Components|Blackboard|SetValueasBool _returnvalue_2 _returnvalue false)
    (else
      (AI|Components|Blackboard|SetValueasBool _returnvalue_2 _returnvalue true))))

(event EventBeginPlay
  (bind _listbehaviortreefoule (Variables|Default|GetListBehaviorTreeFoule))
  (CallFunction|CouleurCorpsAléatoire)
  (AI|RunBehaviorTree (AI|GetAIController self) (Utilities|Array|Get(acopy) _listbehaviortreefoule (Math|Random|RandomInteger (Utilities|Array|Length _listbehaviortreefoule)))))

(fn ConstructionScript)

(fn CouleurCorpsAléatoire
  (bind _bodycolors (Variables|Default|GetBodyColors))
  (Rendering|Material|SetVectorParameterValueonMaterials (Variables|Character|GetMesh) "BodyColor" (Math|Conversions|ToVector(LinearColor) (Utilities|Array|Get(acopy) _bodycolors (Math|Random|RandomInteger (Utilities|Array|Length _bodycolors))))))

(fn FileD'attente
  (params (Numéo%20place :type BP%20File%20Attente%20Object%20Reference))
  (AI|Components|Blackboard|SetValueasVector (AI|GetBlackboard 0) (Utilities|Name|MakeLiteralName "File D'attente") (Transformation|GetWorldLocation (Variables|/Script/Engine.Actor|GetRootComponent Numéo%20place)))
  (Variables|/Game/Environnement/Foule/Elements_Interactif/BP_Echoppe/BP_FileAttente.BP_FileAttente_C|SetPlacePrise Numéo%20place true))

(fn LiébrationPlaceFile
  (params (NuméroPlace :type BP%20File%20Attente%20Object%20Reference))
  (bind _output_get (Variables|Default|SetFiled'attente%20à%20tester (- (Variables|Default|GetFiled'attente%20à%20tester) 1)))
  (AI|Components|Blackboard|SetValueasBool (AI|GetBlackboard 0) (Utilities|Name|MakeLiteralName "GoFile") false)
  (if (>= _output_get 0)
    (AI|Components|Blackboard|SetValueasVector (AI|GetBlackboard 0) (Utilities|Name|MakeLiteralName "File D'attente") (Transformation|GetWorldLocation (Variables|/Script/Engine.Actor|GetRootComponent (Variables|/Script/Engine.ChildActorComponent|GetChildActor (Utilities|Array|Get(acopy) (Variables|/Game/Environnement/Foule/Elements_Interactif/BP_Echoppe/BP_Echoppe.BP_Echoppe_C|GetFileD'attente (Variables|Default|GetEchoppeChoisi)) (Variables|Default|GetFiled'attente%20à%20tester))))))
    (else
      (AI|Components|Blackboard|SetValueasBool (AI|GetBlackboard 0) (Utilities|Name|MakeLiteralName "GoFile") false)
      (AI|Components|Blackboard|SetValueasBool (AI|GetBlackboard 0) (Utilities|Name|MakeLiteralName "Table Libre?") true)
      (Variables|Default|SetFiled'attente%20à%20tester 0))))