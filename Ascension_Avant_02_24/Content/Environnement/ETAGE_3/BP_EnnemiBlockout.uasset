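; BP_EnnemiBlockout is a blockout placeholder for an enemy, labeled in the level with a text render showing its name.
; The construction script and BeginPlay both write the Nom variable to the text, and BeginPlay caches the player's third-person character.
; When that player overlaps the box, a DoOnce gate prints a configurable debug string on the first entry only.
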(event OnComponentBeginOverlap(Box)
  (params (OverlappedComponent :type Primitive%20Component%20Object%20Reference) (OtherActor :type Actor%20Object%20Reference) (OtherComp :type Primitive%20Component%20Object%20Reference) (OtherBodyIndex :type Integer) (bFromSweep :type Boolean) (SweepResult :type Hit%20Result%20Structure%20%28by%20ref%29))
  (if (== OtherActor (Variables|Default|GetJoueur))
    (Utilities|FlowControl|DoOnce false
      (:Completed
        (Development|PrintString (Variables|Default|GetIn%20String) true true "(R=0.000000,G=0.660000,B=1.000000,A=1.000000)" 3.0)))))

(event EventBeginPlay
  (Rendering|Components|TextRender|SetText (Variables|Default|GetTextRender) (Variables|Default|GetNom))
  (bind _asbp_third_person_character (Utilities|Casting|CastToBP_ThirdPersonCharacter (Game|GetPlayerCharacter 0)))
  (Variables|Default|SetJoueur _asbp_third_person_character))

(fn ConstructionScript
  (Rendering|Components|TextRender|SetText (Variables|Default|GetTextRender) (Variables|Default|GetNom)))