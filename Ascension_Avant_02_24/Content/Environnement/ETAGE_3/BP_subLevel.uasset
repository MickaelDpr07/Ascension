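; BP_subLevel is a trigger volume actor that streams sublevels when the player enters its box.
; It caches the BP_ThirdPersonCharacter at BeginPlay and reacts only to that actor's overlap.
; On overlap it loads LevelToLoad, then swaps lighting sublevels by unloading LightToUnload and loading LightToLoad, all without blocking.
; The lighting swap, including the unload, runs only if LightToLoad is valid.
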(event OnComponentBeginOverlap(Box)
  (params (OverlappedComponent :type Primitive%20Component%20Object%20Reference) (OtherActor :type Actor%20Object%20Reference) (OtherComp :type Primitive%20Component%20Object%20Reference) (OtherBodyIndex :type Integer) (bFromSweep :type Boolean) (SweepResult :type Hit%20Result%20Structure%20%28by%20ref%29))
  (if (== OtherActor (Variables|Default|GetJoueur))
    (Utilities|FlowControl|Sequence
      (:then_0
        (if (Utilities|IsValidSoftObjectReference (Variables|Default|GetLevel%20to%20Load))
          (Class|GameplayStatics|LoadStreamLevelbySoftObjectPtr (Variables|Default|GetLevel%20to%20Load) true false)))
      (:then_1
        (if (Utilities|IsValidSoftObjectReference (Variables|Default|GetLight%20to%20Load))
          (Class|GameplayStatics|UnloadStreamLevelbySoftObjectPtr (Variables|Default|GetLight%20to%20Unload) false)
          (Class|GameplayStatics|LoadStreamLevelbySoftObjectPtr (Variables|Default|GetLight%20to%20Load) true false))))))

(event EventBeginPlay
  (bind _returnvalue (Actor|GetActorOfClass "/Game/ThirdPerson/Blueprints/BP_ThirdPersonCharacter.BP_ThirdPersonCharacter_C"))
  (Variables|Default|SetJoueur _returnvalue))

(fn ConstructionScript)