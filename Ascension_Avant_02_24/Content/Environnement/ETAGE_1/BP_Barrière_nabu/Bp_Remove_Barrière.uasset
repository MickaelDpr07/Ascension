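; Trigger actor that removes a BP_Barrière from the level when the player walks into its Box volume.
; On BeginPlay it caches the first BP_Barrière and BP_ThirdPersonCharacter found through GetActorOfClass, so it is not linked to a specific barrier instance.
; When the cached player overlaps the box, it destroys that barrier and then itself, making the removal one-shot.
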(event OnComponentBeginOverlap(Box)
  (params (OverlappedComponent :type Primitive%20Component%20Object%20Reference) (OtherActor :type Actor%20Object%20Reference) (OtherComp :type Primitive%20Component%20Object%20Reference) (OtherBodyIndex :type Integer) (bFromSweep :type Boolean) (SweepResult :type Hit%20Result%20Structure%20%28by%20ref%29))
  (if (== OtherActor (Variables|Default|GetJoueur))
    (Actor|DestroyActor (Variables|Default|GetBarrière))
    (Actor|DestroyActor)))

(event EventBeginPlay
  (bind _returnvalue (Actor|GetActorOfClass "/Game/Environnement/ETAGE_1/BP_Barrière_nabu/BP_Barrière.BP_Barrière_C"))
  (Variables|Default|SetBarrière _returnvalue)
  (bind _returnvalue_2 (Actor|GetActorOfClass "/Game/ThirdPerson/Blueprints/BP_ThirdPersonCharacter.BP_ThirdPersonCharacter_C"))
  (Variables|Default|SetJoueur _returnvalue_2))

(fn ConstructionScript)