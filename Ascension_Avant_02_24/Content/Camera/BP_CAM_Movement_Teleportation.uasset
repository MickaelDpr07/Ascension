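; Camera zone actor that cuts the player's view to its own child-actor camera when the player character enters a trigger.
; The EnableCamera overlap switches the view target and, with StopOnChange, disables player input, which this Blueprint never re-enables.
; The DisableCamera overlap returns the view to the level's BP_Camera_ThirdPerson.
; Construction applies Fov to the child camera, and the input mapping context switching is left disconnected.
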(event OnComponentBeginOverlap(EnableCamera)
  (params (OverlappedComponent :type Primitive%20Component%20Object%20Reference) (OtherActor :type Actor%20Object%20Reference) (OtherComp :type Primitive%20Component%20Object%20Reference) (OtherBodyIndex :type Integer) (bFromSweep :type Boolean) (SweepResult :type Hit%20Result%20Structure%20%28by%20ref%29))
  (if (== OtherActor (Variables|Default|GetPlayer))
    (Variables|Default|SetCharacterInBox true)
    (CallFunction|CameraMovment)
    (if (Variables|Default|GetStopOnChange)
      (Input|DisableInput (Game|GetPlayerCharacter 0) (Game|GetPlayerController 0)))))

(event OnComponentBeginOverlap(DisableCamera)
  (params (OverlappedComponent :type Primitive%20Component%20Object%20Reference) (OtherActor :type Actor%20Object%20Reference) (OtherComp :type Primitive%20Component%20Object%20Reference) (OtherBodyIndex :type Integer) (bFromSweep :type Boolean) (SweepResult :type Hit%20Result%20Structure%20%28by%20ref%29))
  (if (== OtherActor (Variables|Default|GetPlayer))
    (Variables|Default|SetCharacterInBox false)
    (CallFunction|CameraReset)))

(event Custom|CameraMovment
  (if (Variables|Default|GetCharacterInBox)
    (Game|Player|SetViewTargetwithBlend (Game|GetPlayerController 0) (Variables|/Script/Engine.ChildActorComponent|GetChildActor (Variables|Default|GetCamera)) 0.0 "VTBlend_Linear" 0.0 false)
    (bind _asplayer_controller (Utilities|Casting|CastToPlayerController (Pawn|GetController (Variables|Default|GetPlayer))))
    (Utilities|IsValid (PlayerController|LocalPlayerSubsystems|GetEnhancedInputLocalPlayerSubsystem _asplayer_controller))))

(event Custom|CameraReset
  (if (not (Variables|Default|GetCharacterInBox))
    (bind _returnvalue (Actor|GetActorOfClass "/Game/ThirdPerson/Blueprints/BP_Camera_ThirdPerson.BP_Camera_ThirdPerson_C"))
    (Game|Player|SetViewTargetwithBlend (Game|GetPlayerController 0) _returnvalue 0.0 "VTBlend_Linear" 0.0 false)
    (bind _asplayer_controller (Utilities|Casting|CastToPlayerController (Pawn|GetController (Variables|Default|GetPlayer))))
    (Utilities|IsValid (PlayerController|LocalPlayerSubsystems|GetEnhancedInputLocalPlayerSubsystem _asplayer_controller))))

(event EventBeginPlay
  (bind _asbp_third_person_character (Utilities|Casting|CastToBP_ThirdPersonCharacter (Game|GetPlayerCharacter 0)))
  (Variables|Default|SetPlayer _asbp_third_person_character)
  (bind _asgm_exploration (Utilities|Casting|CastToGM_Exploration (Game|GetGameMode)))
  (Variables|Default|SetAs%20GM%20Exploration _asgm_exploration)
  (bind _returnvalue (Actor|GetActorOfClass "/Game/ThirdPerson/Blueprints/BP_Camera_ThirdPerson.BP_Camera_ThirdPerson_C"))
  (Variables|Default|Setcam _returnvalue))

(fn ConstructionScript
  (Camera|SetFieldOfView (Actor|GetComponentbyClass (Variables|/Script/Engine.ChildActorComponent|GetChildActor (Variables|Default|GetCamera)) "/Script/Engine.CameraComponent") (Variables|Default|Getfov)))