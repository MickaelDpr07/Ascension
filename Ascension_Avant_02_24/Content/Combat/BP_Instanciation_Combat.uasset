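; Combat trigger actor that sends the player into the combat level against a specific enemy.
; The construction script looks up the enemy index as a row in the DD_Ennemis data table and sets a text to that enemy's name.
; When the player character overlaps the sphere, it stores the index in the GI_Ascension game instance, carrying it across the level load, then opens the combat level.
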(event OnComponentBeginOverlap(Sphere)
  (params (OverlappedComponent :type Primitive%20Component%20Object%20Reference) (OtherActor :type Actor%20Object%20Reference) (OtherComp :type Primitive%20Component%20Object%20Reference) (OtherBodyIndex :type Integer) (bFromSweep :type Boolean) (SweepResult :type Hit%20Result%20Structure%20%28by%20ref%29))
  ;[1 0 0.1172] Lors Overlap Instanciation Combat, lancement Combat ou Tuto Combat
  (if (== OtherActor (Variables|Default|GetThird%20Person%20Character))
    (Variables|/Game/GI_Ascension.GI_Ascension_C|SetIndex%20Ennemi%20Actuel (Variables|Default|GetGI%20Ascension) (Variables|Default|GetIndex%20Ennemi%20Actu))
    (Game|OpenLevel(byObjectReference) "/Game/ThirdPerson/Maps/LEVEL_Combat.LEVEL_Combat")))

(event EventBeginPlay
  ;[0 1 1] Références
  (bind _asgi_ascension (Utilities|Casting|CastToGI_Ascension (Game|GetGameInstance)))
  (Variables|Default|SetGI%20Ascension _asgi_ascension)
  (bind _asbp_third_person_character (Utilities|Casting|CastToBP_ThirdPersonCharacter (Game|GetPlayerCharacter 0)))
  (Variables|Default|SetThird%20Person%20Character _asbp_third_person_character))

(fn ConstructionScript
  (bind _returnvalue (Utilities|GetDataTableRow "/Game/Combat/Systeme/DD_Ennemis.DD_Ennemis" (Utilities|String|StringToName (Utilities|String|ToString(Integer) (Variables|Default|GetIndex%20Ennemi%20Actu))))
    (:then
      (Rendering|Components|TextRender|SetText (Variables|Default|GetIndexEnnemiActu) (.Nom (Utilities|Struct|BreakSTRUCT_Ennemis _returnvalue))))))