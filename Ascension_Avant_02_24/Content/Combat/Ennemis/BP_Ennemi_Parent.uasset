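; Parent Blueprint for card-combat enemies, loading stats from DD_Ennemis by the current enemy index and showing the name in the combat widget.
; UtilisationCarte casts hard-coded, delayed card sequences per enemy index through GM_Combat; deck creation is an unwired TODO.
; Tick drives a one-second countdown that applies and decrements burn and regeneration through the game mode.
; Card use and the countdown check the game instance's combat pause flag.
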(event Custom|Utilisation%20Carte
  (bind _gi_ascension (Variables|Default|GetGI%20Ascension))
  (bind _index_ennemi_actuel (Variables|/Game/GI_Ascension.GI_Ascension_C|GetIndex%20Ennemi%20Actuel _gi_ascension))
  (if (not (Variables|/Game/GI_Ascension.GI_Ascension_C|GetPause%20du%20Combat%20? (Variables|Default|GetGI%20Ascension)))
    (if (== _index_ennemi_actuel 0)
      (Default|FUseACard (Variables|Default|GetGM%20Combat) 0 0 false)
      (Utilities|FlowControl|Delay 0.2)
      (Default|FUseACard (Variables|Default|GetGM%20Combat) 1 0 false)
      (elif (== _index_ennemi_actuel 1)
        (Default|FUseACard (Variables|Default|GetGM%20Combat) 0 0 false)
        (Utilities|FlowControl|FlipFlop
          (:A
            (Utilities|FlowControl|Delay 0.5)
            (Default|FUseACard (Variables|Default|GetGM%20Combat) 0 0 false))
          (:B
            (Utilities|FlowControl|Delay 2.0)
            (Default|FUseACard (Variables|Default|GetGM%20Combat) 5 0 false)))
        (else
          (Default|FUseACard (Variables|Default|GetGM%20Combat) 1 0 false)
          (Utilities|FlowControl|Delay 0.5)
          (Default|FUseACard (Variables|Default|GetGM%20Combat) 4 0 false)
          (Utilities|FlowControl|Delay 2.1)
          (Default|FUseACard (Variables|Default|GetGM%20Combat) 4 0 false)
          (Utilities|FlowControl|Delay 0.5)
          (Default|FUseACard (Variables|Default|GetGM%20Combat) 5 0 false))))))

(event EventBeginPlay
  (Utilities|FlowControl|Sequence
    (:then_0
      (bind _asgi_ascension (Utilities|Casting|CastToGI_Ascension (Game|GetGameInstance)))
      (Variables|Default|SetGI%20Ascension _asgi_ascension)
      (bind _asgm_combat (Utilities|Casting|CastToGM_Combat (Game|GetGameMode)))
      (Variables|Default|SetGM%20Combat _asgm_combat))
    (:then_1
      (bind _returnvalue (Utilities|GetDataTableRow "/Game/Combat/Systeme/DD_Ennemis.DD_Ennemis" (Utilities|String|StringToName (Utilities|String|ToString(Integer) (Variables|/Game/GI_Ascension.GI_Ascension_C|GetIndex%20Ennemi%20Actuel (Variables|Default|GetGI%20Ascension)))))
        (:then
          (Variables|Default|SetPV (.HP (Utilities|Struct|BreakSTRUCT_Ennemis _returnvalue)))
          (Variables|Default|SetPV%20Max (.HPMax (Utilities|Struct|BreakSTRUCT_Ennemis _returnvalue)))
          (Variables|Default|SetAccreditation (.Accreditation (Utilities|Struct|BreakSTRUCT_Ennemis _returnvalue)))
          (Variables|Default|SetDifficulte (.Difficulte (Utilities|Struct|BreakSTRUCT_Ennemis _returnvalue)))
          (Variables|Default|SetExperience (.Experience (Utilities|Struct|BreakSTRUCT_Ennemis _returnvalue)))
          (bind _output_get (Variables|Default|SetNom (.Nom (Utilities|Struct|BreakSTRUCT_Ennemis _returnvalue))))
          (Rendering|Components|TextRender|SetText (Variables|/Game/Widget/Combat/WB_Combat.WB_Combat_C|GetNomEnnemi (Variables|/Game/GM_Combat.GM_Combat_C|GetWB_Combat (Variables|Default|GetGM%20Combat))) _output_get))))
    (:then_2
      (Variables|Default|SetCompteurTick 1.0))))

(event EventTick
  (params (DeltaSeconds :type Float%20%28single-precision%29))
  (CallFunction|FCompteurTick DeltaSeconds))

(fn ConstructionScript)

(fn FCompteurTick
  (params (Delta%20Time :type Float%20%28double-precision%29))
  (if (not (Variables|/Game/GI_Ascension.GI_Ascension_C|GetPause%20du%20Combat%20? (Variables|Default|GetGI%20Ascension)))
    ;[0.2346 0.4072 0.08022] Compteur de ticks
    (bind _output_get (Variables|Default|SetCompteurTick (- (Variables|Default|GetCompteurTick) Delta%20Time)))
    (if (<= _output_get 0.0)
      (Utilities|FlowControl|Sequence
        (:then_0
          ;[1 0.2917 0.2917] Teste Effet Brulûre
          (if (>= (Variables|Effets|GetBrulure) 0)
            (Default|FBrulure (Variables|Default|GetGM%20Combat) false (Variables|Effets|GetBrulure))
            (Math|Integer|DecrementInt (Variables|Effets|GetBrulure))))
        (:then_1
          ;[0.1661 0.6397 1] Teste Effet Paralyzie
          (if (>= (Variables|Effets|GetRégénération) 0)
            (Default|FRégénération (Variables|Default|GetGM%20Combat) false (Variables|Effets|GetRégénération))
            (Math|Integer|DecrementInt (Variables|Effets|GetRégénération))))
        (:then_2
          ;[0.5783 1 0.1979] Réinitialise le Compteur
          (Variables|Default|SetCompteurTick 1.0))))))