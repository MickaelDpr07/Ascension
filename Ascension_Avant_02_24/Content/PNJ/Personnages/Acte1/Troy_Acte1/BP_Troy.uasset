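; BP_Troy is the Act 1 NPC Troy, who runs a scripted encounter with the player through dialogue and a running follow sequence.
; BeginPlay starts his behavior tree, and the detection overlap locks player input and writes spot and detection keys to the Blackboard.
; Custom events advance Blackboard phases from discussion to running, opening dialogue once with timed cinematic bars.
; Playerfollow auto-walks the player toward Troy with SimpleMoveToActor, restoring input after a delay.
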(event OnComponentBeginOverlap(Detection_Player)
  (params (OverlappedComponent :type Primitive%20Component%20Object%20Reference) (OtherActor :type Actor%20Object%20Reference) (OtherComp :type Primitive%20Component%20Object%20Reference) (OtherBodyIndex :type Integer) (bFromSweep :type Boolean) (SweepResult :type Hit%20Result%20Structure%20%28by%20ref%29))
  (if (== OtherActor (Variables|Default|GetPlayer))
    (AI|Components|Blackboard|SetValueasBool (AI|GetBlackboard 0) (Utilities|Name|MakeLiteralName "Player_Detected") true)
    (AI|Components|Blackboard|SetValueasVector (AI|GetBlackboard 0) (Utilities|Name|MakeLiteralName "Spot_Location") (Transformation|GetWorldLocation (Variables|Default|GetSpot_n1)))
    (Input|DisableInput (Game|GetPlayerCharacter 0) (Game|GetPlayerController 0))))

(event Custom|CoursePoursuiteDiscussion
  (CallFunction|OpenDialog)
  (AI|Components|Blackboard|SetValueasBool (AI|GetBlackboard 0) (Utilities|Name|MakeLiteralName "Course") true)
  (AI|Components|Blackboard|SetValueasBool (AI|GetBlackboard 0) (Utilities|Name|MakeLiteralName "Discussion") false)
  (bind _returnvalue (UserInterface|CreateWidget "/Game/Widget/WB_CameraCinematique.WB_CameraCinematique_C" (Game|GetPlayerController 0)))
  (UserInterface|Viewport|AddtoViewport _returnvalue 0)
  (UserInterface|Animation|PlayAnimation _returnvalue (Variables|/Game/Widget/WB_CameraCinematique.WB_CameraCinematique_C|GetArriveBarre _returnvalue) 0.0 1 "Forward" 1.0 false)
  (Utilities|FlowControl|Delay 9.5)
  (UserInterface|Animation|PlayAnimation _returnvalue (Variables|/Game/Widget/WB_CameraCinematique.WB_CameraCinematique_C|GetFuiteBarre _returnvalue) 0.0 1 "Forward" 1.0 false))

(event Custom|OpenDialog
  (Utilities|FlowControl|DoOnce false
    (:Completed
      (Utilities|Casting|CastToPC_Exploration (Game|GetPlayerController 0))
      (bind _returnvalue (UserInterface|CreateWidget "/Game/PNJ/Dialogues/Widget/WB_Dialogue_Previous.WB_Dialogue_Previous_C" (Game|GetPlayerController 0)))
      (bind _output_get (Variables|Default|SetWB%20Dialogue _returnvalue))
      (UserInterface|Viewport|AddtoViewport _output_get 0)
      (Default|Initialisation (Variables|Default|GetWB%20Dialogue) (Variables|Default|GetDialogue) self (Variables|/Game/GI_Ascension.GI_Ascension_C|GetTroy (Variables|Default|GetGI%20Ascension))))))

(event Custom|EnvoiePositionJoueur
  (AI|Components|Blackboard|SetValueasVector (AI|GetBlackboard 0) (Utilities|Name|MakeLiteralName "Player") (Transformation|GetWorldLocation (Variables|/Script/Engine.Character|GetMesh (Variables|Default|GetPlayer)))))

(event Custom|Lancement%20Discussion
  (AI|Components|Blackboard|SetValueasBool (AI|GetBlackboard 0) (Utilities|Name|MakeLiteralName "Discussion") true)
  (AI|Components|Blackboard|SetValueasBool (AI|GetBlackboard 0) (Utilities|Name|MakeLiteralName "Player_Detected") false))

(event Custom|Player%20follow
  (Variables|/Script/Engine.CharacterMovementComponent|SetMaxWalkSpeed (Variables|/Script/Engine.Character|GetCharacterMovement (Variables|Default|GetPlayer)) 4.5e+02)
  (AI|Navigation|SimpleMovetoActor (Game|GetPlayerController 0) self)
  (Utilities|FlowControl|Delay 1e+01)
  (Input|EnableInput (Game|GetPlayerCharacter 0) (Game|GetPlayerController 0))
  (Variables|/Script/Engine.CharacterMovementComponent|SetMaxWalkSpeed (Variables|/Script/Engine.Character|GetCharacterMovement (Variables|Default|GetPlayer)) 4.5e+02))

(event EventBeginPlay
  (Utilities|FlowControl|Sequence
    (:then_0
      (bind _asgi_ascension (Utilities|Casting|CastToGI_Ascension (Game|GetGameInstance)))
      (Variables|Default|SetGI%20Ascension _asgi_ascension))
    (:then_1
      (bind _asbp_third_person_character (Utilities|Casting|CastToBP_ThirdPersonCharacter (Game|GetPlayerCharacter 0)))
      (Variables|Default|SetPlayer _asbp_third_person_character)
      (AI|RunBehaviorTree (AI|GetAIController self) "/Game/PNJ/Personnages/Acte1/Troy_Acte1/Behavior_Tree/BehaviorTree_Troy.BehaviorTree_Troy")
      (AI|Components|Blackboard|SetValueasVector (AI|GetBlackboard 0) (Utilities|Name|MakeLiteralName "Spot_Nabu") (Transformation|GetWorldLocation (Variables|Default|GetSpot_Nabu))))))

(fn ConstructionScript)