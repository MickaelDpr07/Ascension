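; Dr. Chodo NPC for Act 2, driven by a behavior tree and able to open a dialogue with the player.
; A one-shot event starts the tree, sets the KarlEjected blackboard flag and writes the Destination component's location.
; Rotate yaws the mesh 90 degrees and clears that flag.
; The player's first overlap with Discussion opens the dialogue widget, using a launch ID from the game instance.
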(event OnComponentBeginOverlap(Discussion)
  (params (OverlappedComponent :type Primitive%20Component%20Object%20Reference) (OtherActor :type Actor%20Object%20Reference) (OtherComp :type Primitive%20Component%20Object%20Reference) (OtherBodyIndex :type Integer) (bFromSweep :type Boolean) (SweepResult :type Hit%20Result%20Structure%20%28by%20ref%29))
  (if (== OtherActor (Variables|Default|GetPlayer))
    (CallFunction|OpenDialog)
    (Variables|Default|SetDsicussion? true)))

(event Custom|OpenDialog
  (Utilities|FlowControl|DoOnce false
    (:Completed
      (Utilities|Casting|CastToPC_Exploration (Game|GetPlayerController 0))
      (bind _returnvalue (UserInterface|CreateWidget "/Game/PNJ/Dialogues/Widget/WB_Dialogue_Previous.WB_Dialogue_Previous_C" (Game|GetPlayerController 0)))
      (bind _output_get (Variables|Default|SetDialogue _returnvalue))
      (UserInterface|Viewport|AddtoViewport _output_get 0)
      (Default|Initialisation (Variables|Default|GetDialogue) (Variables|Default|GetDialoguePerso) self (Variables|/Game/GI_Ascension.GI_Ascension_C|GetBob (Variables|Default|GetGI%20Ascension))))))

(event Custom|GoToDestination
  (AI|Components|Blackboard|SetValueasVector (AI|GetBlackboard 0) (Utilities|Name|MakeLiteralName "Destination") (Transformation|GetWorldLocation (Variables|Default|GetDestination))))

(event Custom|Rotate
  (bind _mesh (Variables|Character|GetMesh))
  (bind _returnvalue (Transformation|GetWorldRotation _mesh))
  (Transformation|SetWorldRotation _mesh (Math|Rotator|MakeRotator (.roll _returnvalue) (.pitch _returnvalue) (+ (.yaw _returnvalue) 9e+01)) false false)
  (AI|Components|Blackboard|SetValueasBool (AI|GetBlackboard 0) (Utilities|Name|MakeLiteralName "KarlEjected") false))

(event Custom|Lancement%20behavior%20tree
  (Utilities|FlowControl|DoOnce false
    (:Completed
      (AI|RunBehaviorTree (AI|GetAIController self) "/Game/PNJ/Personnages/Acte2/Dr_Chodo/BehaviorTree/BehaviorTree_Chodo.BehaviorTree_Chodo")
      (AI|Components|Blackboard|SetValueasBool (AI|GetBlackboard 0) (Utilities|Name|MakeLiteralName "KarlEjected") true)
      (CallFunction|GotoDestination))))

(event EventBeginPlay
  (bind _asbp_third_person_character (Utilities|Casting|CastToBP_ThirdPersonCharacter (Game|GetPlayerCharacter 0)))
  (Variables|Default|SetPlayer _asbp_third_person_character)
  (bind _asgi_ascension (Utilities|Casting|CastToGI_Ascension (Game|GetGameInstance)))
  (Variables|Default|SetGI%20Ascension _asgi_ascension))

(fn ConstructionScript)