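; Configurable NPC actor for dialogue and zone blocking, with a floating name pulled from a data table.
; Construction script shows talk and blocking components according to instance flags.
; Talk overlap sets an ACTE22 event in GI_Ascension; blocking overlap checks those events by NPC name to allow passage or walk the player back with input briefly disabled.
; Dialogue is currently placeholder PrintStrings.
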(event OnComponentBeginOverlap(Collision_PNJ_Bloquant?)
  (params (OverlappedComponent :type Primitive%20Component%20Object%20Reference) (OtherActor :type Actor%20Object%20Reference) (OtherComp :type Primitive%20Component%20Object%20Reference) (OtherBodyIndex :type Integer) (bFromSweep :type Boolean) (SweepResult :type Hit%20Result%20Structure%20%28by%20ref%29))
  (bind _gi_ascension (Variables|Référence|GetGI%20Ascension))
  (bind _gi_ascension_2 (Variables|Référence|GetGI%20Ascension))
  ;[1 0.4219 0] PNJ BLOQUANT
  (Utilities|Casting|CastToBP_ThirdPersonCharacter OtherActor)
  (if (Variables|Default|GetBloque%20une%20zone%20?)
    (Utilities|FlowControl|Sequence
      (:then_0
        ;[1 0.7031 0] Lancement Comportement Spécial Blocage PNJ
        (switch Utilities|FlowControl|Switch|SwitchonENUM_PNJ (Variables|Default|GetNom_PNJ)
          (:NewEnumerator2
            (bind _oui___non__ (Default|FLectureEventACTE22 _gi_ascension (Variables|/Game/GI_Ascension.GI_Ascension_C|GetACTE_2_2%20Map _gi_ascension) "NewEnumerator0"))
            (if _oui___non__
              (Variables|Default|SetBloque%20Passage%20? false)
              (Development|PrintString "Vous pouvez passer... Bon combat !" true true "(R=0.000000,G=0.660000,B=1.000000,A=1.000000)" 5.0)))
          (:NewEnumerator3
            (bind _oui___non___2 (Default|FLectureEventACTE22 _gi_ascension_2 (Variables|/Game/GI_Ascension.GI_Ascension_C|GetACTE_2_2%20Map _gi_ascension_2) "NewEnumerator1"))
            (if _oui___non___2
              (Variables|Default|SetBloque%20Passage%20? false)
              (Development|PrintString "Il n'y a perssone... Bien j'y vais" true true "(R=0.000000,G=0.660000,B=1.000000,A=1.000000)" 5.0)))))
      (:then_1
        (CallFunction|BloquePassage (Variables|Default|GetBloque%20Passage%20?))))))

(event OnComponentBeginOverlap(Lancement_Dialogue)
  (params (OverlappedComponent :type Primitive%20Component%20Object%20Reference) (OtherActor :type Actor%20Object%20Reference) (OtherComp :type Primitive%20Component%20Object%20Reference) (OtherBodyIndex :type Integer) (bFromSweep :type Boolean) (SweepResult :type Hit%20Result%20Structure%20%28by%20ref%29))
  ;[1 0.375 0] Lancement dialogue si PNJ en à un
  (Utilities|Casting|CastToBP_ThirdPersonCharacter OtherActor)
  (if (Variables|Default|GetInteraction%20Parler%20?)
    (Development|PrintString "Dialogue qui te donne l'accès à l'entrée des coulisses pour le combat" true true "(R=1.000000,G=0.197663,B=0.000000,A=1.000000)" 1e+01)
    (Utilities|Map|Add (Variables|/Game/GI_Ascension.GI_Ascension_C|GetACTE_2_2%20Map (Variables|Référence|GetGI%20Ascension)) "NewEnumerator0" true)))

(event Custom|Bloque%20Passage
  (params (Passage%20Bloquer%20? :type Boolean))
  ;[1 0.1172 0] CUSTOM EVENT : Bloque Passage
  (if Passage%20Bloquer%20?
    ;;[1 0.02344 0] Ouvre le dialogue du PNJ qui bloque l'accés
    (Development|PrintString "Zone Interdite Dialogue" true true "(R=0.000000,G=0.660000,B=1.000000,A=1.000000)" 5.0)
    ;;[0 1 0.9766] Fais reculer le joueur
    (Input|DisableInput (Game|GetPlayerCharacter 0) (Game|GetPlayerController 0))
    (AI|Navigation|SimpleMovetoLocation (Game|GetPlayerController 0) (Transformation|GetWorldLocation (Variables|Default|GetDestination%20PNJ%20Bloquant)))
    (Utilities|FlowControl|Delay 1.0)
    (Input|EnableInput (Game|GetPlayerCharacter 0) (Game|GetPlayerController 0))))

(event EventBeginPlay
  ;[0 0.3203 1] Référence GI_Ascension
  (bind _asgi_ascension (Utilities|Casting|CastToGI_Ascension (Game|GetGameInstance)))
  (Variables|Référence|SetGI%20Ascension _asgi_ascension))

(fn ConstructionScript
  (bind _collision_pnj_bloquant__ (Variables|Default|GetCollision_PNJ_Bloquant%20?))
  (bind _pnj_row (Variables|Default|GetPNJ_Row))
  (Utilities|FlowControl|Sequence
    (:then_0
      (switch Utilities|FlowControl|Switch|SwitchonENUM_PNJ (Variables|Default|GetNom_PNJ)
        (:NewEnumerator0
          _)
        (:NewEnumerator1
          _)
        (:NewEnumerator2
          _)
        (:NewEnumerator3
          _)
        (:NewEnumerator4
          ;[0.2656 0 1] Si c'est le gérant qui sera dos à nous car il regarde l'arène alors le texte est tourner pour qu'il soit lisible
          (Transformation|AddRelativeRotation (Variables|Default|GetText_Nom_PNJ) "0.000000,180.000000,0.000000" false false))
        (:NewEnumerator6
          _)
        (:NewEnumerator7
          _)
        (:NewEnumerator8
          _))
      ;[1 0 0.5625] Ajout Nom au dessus des PNJs
      (bind _returnvalue (Utilities|GetDataTableRow (.datatable _pnj_row) (.rowname _pnj_row))
        (:then
          (Rendering|Components|TextRender|SetText (Variables|Default|GetText_Nom_PNJ) (.NomPNJ (Utilities|Struct|BreakSTRUCT_Dialogue _returnvalue))))))
    (:then_1
      ;[1 0 0.09375] Rend Visible si le PNJ Bloque une zone
      (if (Variables|Default|GetBloque%20une%20zone%20?)
        (Rendering|SetVisibility _collision_pnj_bloquant__ true false)
        (else
          (Rendering|SetVisibility _collision_pnj_bloquant__ false false))))
    (:then_2
      ;[0.5938 0 1] Rend Visible si on peut Parler au PNJ
      (if (Variables|Default|GetInteraction%20Parler%20?)
        (Rendering|SetVisibility (Variables|Default|GetLancement_Dialogue) true false)
        (else
          (Rendering|SetVisibility (Variables|Default|GetLancement_Dialogue) false false))))))