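; Exploration game mode that sets up default input and the exploration HUD, delayed past any intro cinematic, and runs NPC dialogues.
; Starting a dialogue swaps the HUD, freezes movement and loads the NPC's dialogue table.
; Each advance reads the row indexed by that NPC's GameInstance progress, colours the box by speaker or ends without one.
; "E_" rows trigger events, currently print stubs; "R_" rows offset progress for repeats.
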(event EventBeginPlay
  (Utilities|FlowControl|Sequence
    (:then_0
      ;[1 0.6094 0] Références
      (bind _asgi_ascension (Utilities|Casting|CastToGI_Ascension (Game|GetGameInstance)))
      (Variables|Default|SetGI%20Ascension _asgi_ascension)
      (bind _asbp_third_person_character (Utilities|Casting|CastToBP_ThirdPersonCharacter (Game|GetPlayerCharacter 0)))
      (Variables|Default|SetBP%20Third%20Person _asbp_third_person_character))
    (:then_1
      ;[1 0 0.3047] Changement du Mapping Context lors du lancement de l'exploration
      (bind _aspc_combat (Utilities|Casting|CastToPC_Combat (Game|GetPlayerController 0)))
      (Input|AddMappingContext (PlayerController|LocalPlayerSubsystems|GetEnhancedInputLocalPlayerSubsystem _aspc_combat) "/Game/ThirdPerson/Input/IMC_Default.IMC_Default" 0 "(bIgnoreAllPressedKeysUntilRelease=True,bForceImmediately=False)"))
    (:then_2
      (Variables|/Game/GI_Ascension.GI_Ascension_C|SetEn%20Combat%20? (Variables|Default|GetGI%20Ascension) false))
    (:then_3
      ;[0.1719 1 0] Ouverture du WB_Exploration / Avec un delay si c'est le premier lancement et que donc il y l'animation de l'HUD_Ecriture Cinematique
      (bind _foundwidgets (Widget|GetAllWidgetsOfClass "/Game/Widget/HUD_EcritureCinematique.HUD_EcritureCinematique_C" true))
      (Utilities|IsValid (Utilities|Array|Get(acopy) _foundwidgets)
        (:Is%20Valid
          (Utilities|FlowControl|Delay (Class|WidgetAnimation|GetEndTime (Variables|/Game/Widget/HUD_EcritureCinematique.HUD_EcritureCinematique_C|GetChargements (Utilities|Array|Get(acopy) _foundwidgets)))))
        (:Is%20Not%20Valid
          _))
      (bind _returnvalue (UserInterface|CreateWidget "/Game/Widget/WB_Exploration.WB_Exploration_C"))
      (bind _output_get (Variables|Default|SetWB_Exploration _returnvalue))
      (UserInterface|Viewport|AddtoViewport _output_get 0))))

(fn ConstructionScript)

(fn LancementDialogue
  (params (Nom%20PNJ :type ENUM_PNJ%20Enum :default "NewEnumerator0"))
  (Variables|Default|SetEn%20Dialogue%20? true)
  (Utilities|FlowControl|Sequence
    (:then_0
      ;[0.8281 1 0] Création du widget de dialogue et l'affiche
      (bind _returnvalue (UserInterface|CreateWidget "/Game/PNJ/Dialogues_Final/WB_Final_Dialogues.WB_Final_Dialogues_C"))
      (bind _output_get (Variables|Default|SetWB_Dialogue _returnvalue))
      (UserInterface|Viewport|AddtoViewport _output_get 0)
      ;[0.8516 0 1] Retire les déplacements et le WB_Exploration
      (Widget|RemovefromParent (Variables|Default|GetWB_Exploration))
      (Pawn|Components|CharacterMovement|SetMovementMode (Variables|/Script/Engine.Character|GetCharacterMovement (Variables|Default|GetBP%20Third%20Person)) "MOVE_None" 0))
    (:then_1
      ;[0.6641 1 0] Récupération et sauvegarde du PNJ en cours ainsi que son dialogue
      (bind _output_get_2 (Variables|Default|SetNom%20Actu%20PNJ Nom%20PNJ))
      (bind _returnvalue_2 (Utilities|GetDataTableRow "/Game/PNJ/Dialogues_Final/DT_PNJ_Dialogueable.DT_PNJ_Dialogueable" (Utilities|String|StringToName (Utilities|String|EnumtoString _output_get_2)))
        (:then
          (Variables|Default|SetActu%20Dialogue%20-%20Data%20&%20Avancement (Utilities|Struct|BreakSTRUCT_PNJ_Dialogueable _returnvalue_2))
          (Dialogue|AvancementDialogue))))))

(fn AvancementDialogue
  (bind _wb_dialogue (Variables|Default|GetWB_Dialogue))
  (bind _fondtextaffiché (Variables|/Game/PNJ/Dialogues_Final/WB_Final_Dialogues.WB_Final_Dialogues_C|GetFondTextAffiché _wb_dialogue))
  ;[0 1 0.1797] Récupération du Row du PNJ
  (bind _returnvalue (Utilities|GetDataTableRow (.datatable (Variables|Default|GetActu%20Dialogue%20-%20Data%20&%20Avancement)) (Dialogue|RécupérationIndexRowDialogue))
    (:then
      ;[1 0.2344 0] Split le texte pour voir s'il y un EVENT
      (if (Utilities|Enum|Equal(Enum) "E" (Utilities|Array|Get(acopy) (Utilities|String|ParseIntoArray (Utilities|String|ToString(Text) (.TexteDialogue (Utilities|Struct|BreakSTRUCT_Dialogues_Final _returnvalue))) "_")))
        ;[0.1484 0 1] f_Traitement des Events
        (Dialogue|TraitementDesEvents (Utilities|Array|Get(acopy) (Utilities|String|ParseIntoArray (Utilities|String|ToString(Text) (.TexteDialogue (Utilities|Struct|BreakSTRUCT_Dialogues_Final _returnvalue))) "_") 1))
        (Dialogue|SetRowName(Decalage) 1 :!label _label)
        (elif (Utilities|Enum|Equal(Enum) "R" (Utilities|Array|Get(acopy) (Utilities|String|ParseIntoArray (Utilities|String|ToString(Text) (.TexteDialogue (Utilities|Struct|BreakSTRUCT_Dialogues_Final _returnvalue))) "_")))
          ;[0.4766 1 0] Si dernier dialogue répété
          (Dialogue|SetRowName(Decalage) (Math|Conversions|ToInteger(Byte) (Utilities|Array|Get(acopy) (Utilities|String|ParseIntoArray (Utilities|String|ToString(Text) (.TexteDialogue (Utilities|Struct|BreakSTRUCT_Dialogues_Final _returnvalue))) "_") 1)))
          (else
            ;[0 0.9062 1] MAJ Text et Fond
            (Variables|/Script/UMG.TextBlock|SetText (Variables|/Game/PNJ/Dialogues_Final/WB_Final_Dialogues.WB_Final_Dialogues_C|GetTexte_Affiché (Variables|Default|GetWB_Dialogue)) (.TexteDialogue (Utilities|Struct|BreakSTRUCT_Dialogues_Final _returnvalue)))
            (switch string (Utilities|String|ToString(Text) (.Quiparle? (Utilities|Struct|BreakSTRUCT_Dialogues_Final _returnvalue)))
              (:Default
                ;[1 0 0.9844] Si personne n'es attitré à parler alors met fin au dialogue
                (Dialogue|FinDialogue)
                (goto _label))
              (:PNJ
                (Class|Border|SetBrushColor _fondtextaffiché "(R=0.708000,G=0.219906,B=0.059000,A=1.000000)")
                (goto _label))
              (:Aardus
                (Class|Border|SetBrushColor _fondtextaffiché "(R=0.151959,G=0.530030,B=0.708000,A=1.000000)")
                (goto _label)))))))))

(fn FinDialogue
  (Variables|Default|SetEn%20Dialogue%20? false)
  (Widget|RemovefromParent (Variables|Default|GetWB_Dialogue))
  ;[0.8516 0 1] Remet les déplacements & le WB_Exploration
  (UserInterface|Viewport|AddtoViewport (Variables|Default|GetWB_Exploration) 0)
  (Pawn|Components|CharacterMovement|SetMovementMode (Variables|/Script/Engine.Character|GetCharacterMovement (Variables|Default|GetBP%20Third%20Person)) "MOVE_Walking" 0))

(fn RécupérationIndexRowDialogue
  (bind _gi_ascension (Variables|Default|GetGI%20Ascension))
  (bind _pnj_avancement_dialogue (Variables|/Game/GI_Ascension.GI_Ascension_C|GetPNJ_Avancement_Dialogue _gi_ascension))
  (bind _keys (Utilities|Map|Keys _pnj_avancement_dialogue))
  (bind _values (Utilities|Map|Values _pnj_avancement_dialogue))
  (return (Utilities|String|StringToName (Utilities|String|ToString(Integer) (Utilities|Array|Get(acopy) _values (Utilities|Array|FindItem _keys (Variables|Default|GetNom%20Actu%20PNJ)))))))

(fn SetRowName(Decalage)
  (params (Decalage%20Row :type Integer))
  (bind _gi_ascension (Variables|Default|GetGI%20Ascension))
  (bind _pnj_avancement_dialogue (Variables|/Game/GI_Ascension.GI_Ascension_C|GetPNJ_Avancement_Dialogue _gi_ascension))
  (bind _keys (Utilities|Map|Keys _pnj_avancement_dialogue))
  (bind _values (Utilities|Map|Values _pnj_avancement_dialogue))
  (Utilities|Map|Add (Variables|/Game/GI_Ascension.GI_Ascension_C|GetPNJ_Avancement_Dialogue (Variables|Default|GetGI%20Ascension)) (Variables|Default|GetNom%20Actu%20PNJ) (+ (Utilities|Array|Get(acopy) _values (Utilities|Array|FindItem _keys (Variables|Default|GetNom%20Actu%20PNJ))) Decalage%20Row))
  (return))

(fn TraitementDesEvents
  (params (Nom_Event :type String))
  (switch string Nom_Event
    (:Mouvement
      (Development|PrintString "Mouvement"))
    (:AmeliorationPerso
      (Development|PrintString "AmeliorationPerso"))
    (:Deck
      (Development|PrintString "Deck"))))