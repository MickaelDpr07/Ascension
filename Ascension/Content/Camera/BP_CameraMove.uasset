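; BP_CameraMove is a trigger volume that changes the third-person camera's distance when the player enters it.
; BeginPlay caches the player character and the BP_Camera_ThirdPerson actor, and stores and prints the camera's starting DistanceX.
; When the player's capsule begins overlapping the Box, the camera's DistanceX takes this actor's own DistanceX value.
; The stored default is never restored, as no end-overlap handling exists.
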(event OnComponentBeginOverlap(Box)
  (params (OverlappedComponent :type Primitive%20Component%20Object%20Reference) (OtherActor :type Actor%20Object%20Reference) (OtherComp :type Primitive%20Component%20Object%20Reference) (OtherBodyIndex :type Integer) (bFromSweep :type Boolean) (SweepResult :type Hit%20Result%20Structure%20%28by%20ref%29))
  (if (== OtherComp (Variables|/Script/Engine.Character|GetCapsuleComponent (Variables|Default|GetJoueur)))
    (Variables|/Game/ThirdPerson/Blueprints/BP_Camera_ThirdPerson.BP_Camera_ThirdPerson_C|SetDistance%20X (Variables|Default|GetCam) (Variables|Default|GetDistance%20X))))

(event EventBeginPlay
  (bind _asbp_third_person_character (Utilities|Casting|CastToBP_ThirdPersonCharacter (Game|GetPlayerCharacter 0)))
  (Variables|Default|SetJoueur _asbp_third_person_character)
  (bind _returnvalue (Actor|GetActorOfClass "/Game/ThirdPerson/Blueprints/BP_Camera_ThirdPerson.BP_Camera_ThirdPerson_C"))
  (Variables|Default|SetCam _returnvalue)
  (bind _output_get (Variables|Default|SetxDefault (Variables|/Game/ThirdPerson/Blueprints/BP_Camera_ThirdPerson.BP_Camera_ThirdPerson_C|GetDistance%20X (Variables|Default|GetCam))))
  (Development|PrintString (Utilities|String|ToString(Float) _output_get)))

(fn ConstructionScript)