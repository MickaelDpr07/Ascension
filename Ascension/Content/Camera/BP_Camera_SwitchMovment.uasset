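; Camera switch actor that moves the player's view between the third-person camera and entrance and exit child-actor cameras.
; Each entrance overlap blends to the entrance camera and flip-flops CharacterEnter; the exit overlap blends to the exit camera and sets it true.
; While true, Tick moves the entrance camera with the player, copying third-person height and rotation.
; While false, Tick reasserts the third-person view every frame.
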(event OnComponentBeginOverlap(Collision_Entree)
  (params (OverlappedComponent :type Primitive%20Component%20Object%20Reference) (OtherActor :type Actor%20Object%20Reference) (OtherComp :type Primitive%20Component%20Object%20Reference) (OtherBodyIndex :type Integer) (bFromSweep :type Boolean) (SweepResult :type Hit%20Result%20Structure%20%28by%20ref%29))
  (if (== OtherComp (Variables|/Script/Engine.Character|GetCapsuleComponent (Variables|Default|GetJoueur)))
    (Game|Player|SetViewTargetwithBlend (Game|GetPlayerController 0) (Variables|/Script/Engine.ChildActorComponent|GetChildActor (Variables|Default|GetCamera_Entree)) 0.0 "VTBlend_Linear" 0.0 false)
    (Utilities|FlowControl|FlipFlop
      (:A
        (Variables|Default|SetCharacter_enter true))
      (:B
        (Variables|Default|SetCharacter_enter false)))))

(event OnComponentBeginOverlap(Collision_Sortie)
  (params (OverlappedComponent :type Primitive%20Component%20Object%20Reference) (OtherActor :type Actor%20Object%20Reference) (OtherComp :type Primitive%20Component%20Object%20Reference) (OtherBodyIndex :type Integer) (bFromSweep :type Boolean) (SweepResult :type Hit%20Result%20Structure%20%28by%20ref%29))
  (if (== OtherComp (Variables|/Script/Engine.Character|GetCapsuleComponent (Variables|Default|GetJoueur)))
    (Game|Player|SetViewTargetwithBlend (Game|GetPlayerController 0) (Variables|/Script/Engine.ChildActorComponent|GetChildActor (Variables|Default|GetCamera_Sortie)) 0.0 "VTBlend_Linear" 0.0 false)
    (Variables|Default|SetCharacter_enter true)))

(event EventBeginPlay
  (bind _returnvalue (Actor|GetActorOfClass "/Game/Camera/Bp_Camera_Couloir.Bp_Camera_Couloir_C"))
  (Variables|Default|SetCamera_Couloir _returnvalue)
  (bind _asbp_third_person_character (Utilities|Casting|CastToBP_ThirdPersonCharacter (Game|GetPlayerCharacter 0)))
  (Variables|Default|SetJoueur _asbp_third_person_character)
  (bind _returnvalue_2 (Actor|GetActorOfClass "/Game/ThirdPerson/Blueprints/BP_Camera_ThirdPerson.BP_Camera_ThirdPerson_C"))
  (Variables|Default|SetCamera_Personnage _returnvalue_2))

(event EventTick
  (params (DeltaSeconds :type Float%20%28single-precision%29))
  (bind _joueur (Variables|Default|GetJoueur))
  (bind _camera_entree (Variables|Default|GetCamera_Entree))
  (bind _childactor (Variables|/Script/Engine.ChildActorComponent|GetChildActor _camera_entree))
  (bind _mesh (Variables|/Script/Engine.Character|GetMesh _joueur))
  (bind _returnvalue (Transformation|GetWorldLocation _mesh))
  (if (Variables|Default|GetCharacter_enter)
    (Utilities|FlowControl|Sequence
      (:then_0
        (Transformation|SetActorLocation _childactor (Math|Vector|MakeVector (- (.x _returnvalue) 4.5e+02) (.y _returnvalue) (+ (.z _returnvalue) (Variables|/Game/ThirdPerson/Blueprints/BP_Camera_ThirdPerson.BP_Camera_ThirdPerson_C|GetDistance%20Z (Variables|Default|GetCamera_Personnage)))) false false))
      (:then_1
        (Transformation|SetActorRotation _childactor (Transformation|GetWorldRotation (Variables|/Game/ThirdPerson/Blueprints/BP_Camera_ThirdPerson.BP_Camera_ThirdPerson_C|GetCamera (Variables|Default|GetCamera_Personnage))))))
    (else
      (Game|Player|SetViewTargetwithBlend (Game|GetPlayerController 0) (Variables|Default|GetCamera_Personnage) 0.0 "VTBlend_Linear" 0.0 false))))

(fn ConstructionScript)