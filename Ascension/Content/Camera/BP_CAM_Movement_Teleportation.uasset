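; BP_CAM_Movement_Teleportation is a camera zone that switches the player's view to its child-actor camera.
; Overlapping the EnableCamera trigger sets that view without a blend time and can disable input, with no re-enable here.
; The DisableCamera trigger restores the level's BP_Camera_ThirdPerson.
; The construction script applies Fov to the child camera; input mapping-context switching is unwired, and debug prints remain.
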(event OnComponentBeginOverlap(EnableCamera)
  (params (OverlappedComponent :type Primitive%20Component%20Object%20Reference) (OtherActor :type Actor%20Object%20Reference) (OtherComp :type Primitive%20Component%20Object%20Reference) (OtherBodyIndex :type Integer) (bFromSweep :type Boolean) (SweepResult :type Hit%20Result%20Structure%20%28by%20ref%29))
  (if (== OtherComp (Variables|/Script/Engine.Character|GetCapsuleComponent (Variables|Default|GetPlayer)))
    (Variables|Default|SetCharacterInBox true)
    (CallFunction|CameraMovment)
    (Development|PrintString "Hello")
    (if (Variables|Default|GetStopOnChange)
      (Input|DisableInput (Game|GetPlayerCharacter 0) (Game|GetPlayerController 0)))))

(event OnComponentBeginOverlap(DisableCamera)
  (params (OverlappedComponent :type Primitive%20Component%20Object%20Reference) (OtherActor :type Actor%20Object%20Reference) (OtherComp :type Primitive%20Component%20Object%20Reference) (OtherBodyIndex :type Integer) (bFromSweep :type Boolean) (SweepResult :type Hit%20Result%20Structure%20%28by%20ref%29))
  (if (== OtherComp (Variables|/Script/Engine.Character|GetCapsuleComponent (Variables|Default|GetPlayer)))
    (Variables|Default|SetCharacterInBox false)
    (CallFunction|CameraReset)
    (Development|PrintString "Bye")))

(event Custom|CameraMovment
  (if (Variables|Default|GetCharacterInBox)
    (Game|Player|SetViewTargetwithBlend (Game|GetPlayerController 0) (Variables|/Script/Engine.ChildActorComponent|GetChildActor (Variables|Default|GetCamera)) 0.0 "VTBlend_Linear" 0.0 false)
    (bind _asplayer_controller (Utilities|Casting|CastToPlayerController (Pawn|GetController (Variables|Default|GetPlayer))))
    (Utilities|IsValid (PlayerController|LocalPlayerSubsystems|GetEnhancedInputLocalPlayerSubsystem _asplayer_controller))))

(event Custom|CameraReset
  (if (not (Variables|Default|GetCharacterInBox))
    (Game|Player|SetViewTargetwithBlend (Game|GetPlayerController 0) (Variables|Default|GetCam) 0.0 "VTBlend_Linear" 0.0 false)
    (bind _asplayer_controller (Utilities|Casting|CastToPlayerController (Pawn|GetController (Variables|Default|GetPlayer))))
    (Utilities|IsValid (PlayerController|LocalPlayerSubsystems|GetEnhancedInputLocalPlayerSubsystem _asplayer_controller))))

(event EventBeginPlay
  (bind _asbp_third_person_character (Utilities|Casting|CastToBP_ThirdPersonCharacter (Game|GetPlayerCharacter 0)))
  (Variables|Default|SetPlayer _asbp_third_person_character)
  (bind _returnvalue (Actor|GetActorOfClass "/Game/ThirdPerson/Blueprints/BP_Camera_ThirdPerson.BP_Camera_ThirdPerson_C"))
  (Variables|Default|SetCam _returnvalue))

(fn ConstructionScript
  (Camera|SetFieldOfView (Actor|GetComponentbyClass (Variables|/Script/Engine.ChildActorComponent|GetChildActor (Variables|Default|GetCamera)) "/Script/Engine.CameraComponent") (Variables|Default|Getfov)))