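; Bp_Cam_Central is a fixed camera actor that becomes the player's view and keeps aimed at the third-person character.
; On BeginPlay it finds BP_ThirdPersonCharacter, stores it, and sets itself as the view target of player controller 0.
; Every Tick it rotates its camera component toward the character's root position using FindLookAtRotation, with no smoothing.
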(event EventBeginPlay
  (bind _returnvalue (Actor|GetActorOfClass "/Game/ThirdPerson/Blueprints/BP_ThirdPersonCharacter.BP_ThirdPersonCharacter_C"))
  (Variables|Default|SetPlayer _returnvalue)
  (Game|Player|SetViewTargetwithBlend (Game|GetPlayerController 0) self 0.0 "VTBlend_Linear" 0.0 false))

(event EventTick
  (params (DeltaSeconds :type Float%20%28single-precision%29))
  (Transformation|SetWorldRotation (Variables|Default|GetCamera) (Math|Rotator|FindLookatRotation (Transformation|GetWorldLocation (Variables|Default|GetCamera)) (Transformation|GetWorldLocation (Variables|/Script/Engine.Actor|GetRootComponent (Variables|Default|GetPlayer)))) false false))

(fn ConstructionScript)