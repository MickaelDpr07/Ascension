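; Freight elevator with a configurable platform mesh and height that alternately rises and descends each time the player enters its collision.
; The overlap switches to a child camera actor, and a DoOnce with FlipFlop locks input while MoveComponentTo moves the platform.
; If flagged as the combat arena lift and its GI_Ascension event is unset, it shows the three-fight objective, records the event, destroys its trigger and descends.
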(event OnComponentBeginOverlap(Collision)
  (params (OverlappedComponent :type Primitive%20Component%20Object%20Reference) (OtherActor :type Actor%20Object%20Reference) (OtherComp :type Primitive%20Component%20Object%20Reference) (OtherBodyIndex :type Integer) (bFromSweep :type Boolean) (SweepResult :type Hit%20Result%20Structure%20%28by%20ref%29))
  (bind _gi_ascension (Variables|Default|GetGI%20Ascension))
  (bind _camera (Variables|Default|GetCamera))
  (bind _childactor (Variables|/Script/Engine.ChildActorComponent|GetChildActor _camera))
  (Utilities|Casting|CastToBP_ThirdPersonCharacter OtherActor)
  (Game|Player|SetViewTargetwithBlend (Game|GetPlayerController 0) _childactor 0.0 "VTBlend_Linear" 0.0 false)
  (bind _asbp_camera_shop (Utilities|Casting|CastToBp_Camera_Shop _childactor))
  (Camera|SetFieldOfView (Variables|/Game/Camera/Bp_Camera_Shop.Bp_Camera_Shop_C|GetCamera _asbp_camera_shop) 1e+02)
  ;[0 1 0.2734] Mouvement de l'ascenseur
  (Utilities|FlowControl|DoOnce false :!label _label
    (:Completed
      (Input|DisableInput (Game|GetPlayerCharacter 0) (Game|GetPlayerController 0))
      (Utilities|FlowControl|FlipFlop
        (:A
          ;;[0.1953 1 0] Mouvement Monter
          (Components|MoveComponentTo (Variables|Default|GetPlateforme) (Math|Vector|MakeVector 0.0 0.0 (Variables|Default|GetHauteur)) "0, 0, 0" false false 3.0 false)
          ;;[1 0.2578 0] Test si l'ascenseur est celui de l'arène et si l'arène à était gagner
          (bind _oui___non__ (Default|FLectureEventACTE22 _gi_ascension (Variables|/Game/GI_Ascension.GI_Ascension_C|GetACTE_2_2%20Map _gi_ascension) "NewEnumerator1" :!label _label_2))
          (if (and (not _oui___non__) (Variables|Default|GetArèneDeCombat%20?))
            ;[1 0 0.375] Les 3 COMBATS VICTORIEUX
            (Development|PrintString "Effectuer les 3 combats de l'arènes et victoires sur chacuns" true true "(R=0.000000,G=0.660000,B=1.000000,A=1.000000)" 1e+01)
            ;;[0.4766 0 1] Actions si l'ascenseur est celui de l'arène
            (Utilities|Map|Add (Variables|/Game/GI_Ascension.GI_Ascension_C|GetACTE_2_2%20Map (Variables|Default|GetGI%20Ascension)) "NewEnumerator1" true)
            (Components|DestroyComponent (Variables|Default|GetCollision))
            (Utilities|FlowControl|Delay 2.0)
            ;;[0.1953 1 0] Mouvement Descendre
            (Components|MoveComponentTo (Variables|Default|GetPlateforme) "0, 0, 0" "0, 0, 0" false false 3.0 false :!label _label_3)
            (goto _label_2)
            (else
              _)))
        (:B
          (goto _label_3)))
      (Input|EnableInput (Game|GetPlayerCharacter 0) (Game|GetPlayerController 0))
      (goto _label Reset))))

(event EventBeginPlay
  ;[0 0.0625 1] Référence Gi_Ascension
  (bind _asgi_ascension (Utilities|Casting|CastToGI_Ascension (Game|GetGameInstance)))
  (Variables|Default|SetGI%20Ascension _asgi_ascension))

(fn ConstructionScript
  ;[0 0.1797 1] Pour pouvoir changer le static mesh dans la scène
  (Components|StaticMesh|SetStaticMesh (Variables|Default|GetPlateforme) (Variables|Default|GetMesh%20Plateforme)))