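; Base Blueprint for a talkable NPC in exploration, showing its enum-driven name as world text rotated once toward the main camera shortly after BeginPlay.
; Its collision box toggles the talk prompt and button, registers the NPC with GM_Exploration on entry, and sets the current interaction type, with certain NPCs (Nano-Nurse upgrade) getting a separate type.
; NePourraPlusParler destroys the collision box to permanently disable dialogue.
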(event OnComponentBeginOverlap(CollisionBox)
  (params (OverlappedComponent :type Primitive%20Component%20Object%20Reference) (OtherActor :type Actor%20Object%20Reference) (OtherComp :type Primitive%20Component%20Object%20Reference) (OtherBodyIndex :type Integer) (bFromSweep :type Boolean) (SweepResult :type Hit%20Result%20Structure%20%28by%20ref%29))
  (bind _nom_pnj (Variables|Default|GetNom%20PNJ))
  (bind _gm_exploration (Variables|Default|GetGM%20Exploration))
  (Development|SetHiddeninGame (Variables|Default|GetTXT%20Pour%20discuter) false false)
  (Variables|/Game/GM_Exploration.GM_Exploration_C|SetLe%20PNJ%20qui%20Dialogue _gm_exploration self)
  ;[1 0.8906 0] Test si on va lancer le Widget Amélioration (Nano-Nurse)
  (if (or (Utilities|Enum|Equal(Enum) "NewEnumerator7" _nom_pnj) (Utilities|Enum|Equal(Enum) _nom_pnj "NewEnumerator1"))
    (Variables|/Game/GM_Exploration.GM_Exploration_C|SetENUM_Interaction_Actu _gm_exploration "NewEnumerator5")
    (else
      (Variables|/Game/GM_Exploration.GM_Exploration_C|SetENUM_Interaction_Actu _gm_exploration "NewEnumerator2"))))

(event OnComponentEndOverlap(CollisionBox)
  (params (OverlappedComponent :type Primitive%20Component%20Object%20Reference) (OtherActor :type Actor%20Object%20Reference) (OtherComp :type Primitive%20Component%20Object%20Reference) (OtherBodyIndex :type Integer))
  (Development|SetHiddeninGame (Variables|Default|GetTXT%20Pour%20discuter) true false)
  (Variables|/Game/GM_Exploration.GM_Exploration_C|SetENUM_Interaction_Actu (Variables|Default|GetGM%20Exploration) "NewEnumerator1"))

(event EventBeginPlay
  ;[0.007812 0 1] Références
  (bind _asgm_exploration (Utilities|Casting|CastToGM_Exploration (Game|GetGameMode)))
  (Variables|Default|SetGM%20Exploration _asgm_exploration)
  (bind _outactors (Actor|GetAllActorsOfClass "/Game/Camera/BP_MAIN_CAM.BP_MAIN_CAM_C"))
  (bind _output_get (Variables|Default|SetMAIN%20CAM (Utilities|Array|Get(acopy) _outactors)))
  ;[1 0 0.3047] Set Text Face MAIN CAM
  ;;[1 0 0.04822] DELAY pour que la CAM est le temps de changer de position
  (Utilities|FlowControl|Delay 0.1)
  (Transformation|SetWorldRotation (Variables|Default|GetTXT%20Nom%20PNJ) (Math|Rotator|FindLookatRotation (Transformation|GetWorldLocation (Variables|Default|GetTXT%20Nom%20PNJ)) (Transformation|GetActorLocation _output_get)) false false))

(fn ConstructionScript
  (Rendering|Components|TextRender|SetText (Variables|Default|GetTXT%20Nom%20PNJ) (Utilities|Text|ToText(String) (Utilities|String|EnumtoString (Variables|Default|GetNom%20PNJ)))))

(fn NePourraPlusParler
  (Components|DestroyComponent (Variables|Default|GetCollision%20Box)))