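; BP_Nabu is an Act 1 NPC that starts a dialogue when the player walks into its trigger sphere.
; BeginPlay caches the GI_Ascension game instance and the BP_ThirdPersonCharacter player for later use.
; The overlap opens a WB_Dialogue widget through a DoOnce that is never reset, provided the controller is PC_Exploration.
; The widget is initialised with this NPC, its dialogue table and the game instance's Nabu value as launch ID.
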(event OnComponentBeginOverlap(Sphere)
  (params (OverlappedComponent :type Primitive%20Component%20Object%20Reference) (OtherActor :type Actor%20Object%20Reference) (OtherComp :type Primitive%20Component%20Object%20Reference) (OtherBodyIndex :type Integer) (bFromSweep :type Boolean) (SweepResult :type Hit%20Result%20Structure%20%28by%20ref%29))
  (if (== OtherActor (Variables|Default|GetPlayer))
    (CallFunction|OpenDialog)))

(event Custom|OpenDialog
  (Utilities|FlowControl|DoOnce false
    (:Completed
      (Utilities|Casting|CastToPC_Exploration (Game|GetPlayerController 0))
      (bind _returnvalue (UserInterface|CreateWidget "/Game/PNJ/Dialogues/Widget/WB_Dialogue.WB_Dialogue_C" (Game|GetPlayerController 0)))
      (bind _output_get (Variables|Default|SetDialogue _returnvalue))
      (UserInterface|Viewport|AddtoViewport _output_get 0)
      (Default|Initialisation (Variables|Default|GetDialogue) (Variables|Default|GetDialoguePerso) self (Variables|/Game/GI_Ascension.GI_Ascension_C|GetNabu (Variables|Default|GetGI%20Ascension))))))

(event EventBeginPlay
  (Utilities|FlowControl|Sequence
    (:then_0
      (bind _asgi_ascension (Utilities|Casting|CastToGI_Ascension (Game|GetGameInstance)))
      (Variables|Default|SetGI%20Ascension _asgi_ascension))
    (:then_1
      (bind _asbp_third_person_character (Utilities|Casting|CastToBP_ThirdPersonCharacter (Game|GetPlayerCharacter 0)))
      (Variables|Default|SetPlayer _asbp_third_person_character))))

(fn ConstructionScript)