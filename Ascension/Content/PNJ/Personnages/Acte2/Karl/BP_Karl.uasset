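; Act 2 NPC Karl: runs a scripted ejection sequence driven by a behavior tree.
; Overlapping Ejection_Karl freezes the player and sets the blackboard destination and detection flag.
; The Ragdoll event launches Karl with physics, restores player movement, starts Chodo's behavior tree and opens a one-time dialogue keyed by the game instance.
; A second trigger, DeleteKarl, destroys the actor when the player character overlaps it.
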(event OnComponentBeginOverlap(Ejection_Karl)
  (params (OverlappedComponent :type Primitive%20Component%20Object%20Reference) (OtherActor :type Actor%20Object%20Reference) (OtherComp :type Primitive%20Component%20Object%20Reference) (OtherBodyIndex :type Integer) (bFromSweep :type Boolean) (SweepResult :type Hit%20Result%20Structure%20%28by%20ref%29))
  (if (== OtherActor (Variables|Default|GetPlayer))
    (Pawn|Components|CharacterMovement|SetMovementMode (Variables|/Script/Engine.Character|GetCharacterMovement (Variables|Default|GetPlayer)) "MOVE_None" 0)
    (AI|Components|Blackboard|SetValueasVector (AI|GetBlackboard 0) (Utilities|Name|MakeLiteralName "Destination") (Transformation|GetWorldLocation (Variables|Default|GetDestination)))
    (AI|Components|Blackboard|SetValueasBool (AI|GetBlackboard 0) (Utilities|Name|MakeLiteralName "PlayerDetected") true)))

(event OnComponentBeginOverlap(DeleteKarl)
  (params (OverlappedComponent :type Primitive%20Component%20Object%20Reference) (OtherActor :type Actor%20Object%20Reference) (OtherComp :type Primitive%20Component%20Object%20Reference) (OtherBodyIndex :type Integer) (bFromSweep :type Boolean) (SweepResult :type Hit%20Result%20Structure%20%28by%20ref%29))
  (Utilities|Casting|CastToBP_ThirdPersonCharacter OtherActor)
  (Development|PrintString "Hello")
  (Actor|DestroyActor))

(event Custom|Ragdoll
  (bind _mesh (Variables|Character|GetMesh))
  (Physics|SetSimulatePhysics (Variables|Character|GetMesh) true)
  (Physics|AddImpulse _mesh (Math|Conversions|ToVector(Float) (* (.x (Math|Vector|GetForwardVector _mesh)) 2.5e+02)) "None" true)
  (Pawn|Components|CharacterMovement|SetMovementMode (Variables|/Script/Engine.Character|GetCharacterMovement (Variables|Default|GetPlayer)) "MOVE_Walking" 0)
  (Collision|SetCollisionEnabled (Variables|Collision|GetCapsuleComponent) "NoCollision")
  (Default|LancementBehaviorTree (Variables|Default|GetChodo))
  (CallFunction|OpenDialog))

(event Custom|OpenDialog
  (Utilities|FlowControl|DoOnce false
    (:Completed
      (Utilities|Casting|CastToPC_Exploration (Game|GetPlayerController 0))
      (bind _returnvalue (UserInterface|CreateWidget "/Game/PNJ/Dialogues/Widget/WB_Dialogue_Previous.WB_Dialogue_Previous_C" (Game|GetPlayerController 0)))
      (bind _output_get (Variables|Default|SetDialogue _returnvalue))
      (UserInterface|Viewport|AddtoViewport _output_get 0)
      (Default|Initialisation (Variables|Default|GetDialogue) (Variables|Default|GetDialoguePerso) self (Variables|/Game/GI_Ascension.GI_Ascension_C|GetBob (Variables|Default|GetGI%20Ascension))))))

(event EventBeginPlay
  (bind _asbp_third_person_character (Utilities|Casting|CastToBP_ThirdPersonCharacter (Game|GetPlayerCharacter 0)))
  (Variables|Default|SetPlayer _asbp_third_person_character)
  (AI|RunBehaviorTree (AI|GetAIController self) "/Game/PNJ/Personnages/Acte2/Karl/Behavior_Tree/BehaviorTreeKarl.BehaviorTreeKarl")
  (bind _returnvalue (Actor|GetActorOfClass "/Game/PNJ/Personnages/Acte2/Dr_Chodo/BP_Chodo.BP_Chodo_C"))
  (Variables|Default|SetChodo _returnvalue)
  (bind _asgi_ascension (Utilities|Casting|CastToGI_Ascension (Game|GetGameInstance)))
  (Variables|Default|SetGI%20Ascension _asgi_ascension))

(fn ConstructionScript)