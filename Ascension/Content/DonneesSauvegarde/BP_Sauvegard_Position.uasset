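; BP_Sauvegard_Position is a checkpoint trigger that saves the player's position in the level.
; On BeginPlay it caches the third-person player character and the GI_Ascension game instance.
; When the player first overlaps its Collision component, a DoOnce stores the character's transform in the game instance's PositionJoueurSaved and prints a confirmation message.
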(event OnComponentBeginOverlap(Collision)
  (params (OverlappedComponent :type Primitive%20Component%20Object%20Reference) (OtherActor :type Actor%20Object%20Reference) (OtherComp :type Primitive%20Component%20Object%20Reference) (OtherBodyIndex :type Integer) (bFromSweep :type Boolean) (SweepResult :type Hit%20Result%20Structure%20%28by%20ref%29))
  (if (== OtherActor (Variables|Default|GetPlayer))
    (Utilities|FlowControl|DoOnce false
      (:Completed
        ;[1 0 0.9375] Sauvegarde Lieu dans le Level
        (Variables|/Game/GI_Ascension.GI_Ascension_C|SetPositionJoueur_Saved (Variables|Default|GetGI%20Ascension) (Transformation|GetActorTransform (Variables|Default|GetPlayer)))
        (Development|PrintString "Sauvegarde Position")))))

(event EventBeginPlay
  (bind _asbp_third_person_character (Utilities|Casting|CastToBP_ThirdPersonCharacter (Game|GetPlayerCharacter 0)))
  (Variables|Default|SetPlayer _asbp_third_person_character)
  (bind _asgi_ascension (Utilities|Casting|CastToGI_Ascension (Game|GetGameInstance)))
  (Variables|Default|SetGI%20Ascension _asgi_ascension))

(fn ConstructionScript)