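; Secret door actor that slides along world X when the player interacts inside its trigger box, then slides back.
; A 0.1-second looping timer polls the character's Interract flag and the box overlap, ignored while Enmouvement is set.
; One timeline drives the opening; a delay from its Update reverses a second timeline, whose Update clears Enmouvement.
; World Y and Z are hard-coded, and the stored start position Posdepart is unused.
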(event OnComponentBeginOverlap(Box)
  (params (OverlappedComponent :type Primitive%20Component%20Object%20Reference) (OtherActor :type Actor%20Object%20Reference) (OtherComp :type Primitive%20Component%20Object%20Reference) (OtherBodyIndex :type Integer) (bFromSweep :type Boolean) (SweepResult :type Hit%20Result%20Structure%20%28by%20ref%29))
  (Variables|Default|SetDans%20la%20box true))

(event OnComponentEndOverlap(Box)
  (params (OverlappedComponent :type Primitive%20Component%20Object%20Reference) (OtherActor :type Actor%20Object%20Reference) (OtherComp :type Primitive%20Component%20Object%20Reference) (OtherBodyIndex :type Integer))
  (Variables|Default|SetDans%20la%20box false))

(event Custom|CustomEvent
  (if (not (Variables|Default|GetEnmouvement))
    (if (and (Variables|/Game/ThirdPerson/Blueprints/BP_ThirdPersonCharacter.BP_ThirdPersonCharacter_C|GetInterract (Variables|Default|GetJoueru)) (Variables|Default|GetDans%20la%20box))
      (Variables|Default|SetEnmouvement true)
      (bind _newtrack_0 (Timeline|Timeline PlayFromStart)
        (:Update
          (Transformation|SetWorldLocation (Variables|Default|GetDefaultSceneRoot) (Math|Vector|MakeVector (.x _newtrack_0) 16735.0 -910.999878) false false)
          (Utilities|FlowControl|Delay 5.0)
          (bind _newtrack_0_2 (Timeline|Timeline_0 ReverseFromEnd)
            (:Update
              (Transformation|SetWorldLocation (Variables|Default|GetDefaultSceneRoot) (Math|Vector|MakeVector (.x _newtrack_0_2) 16735.0 -910.999878) false false)
              (Variables|Default|SetEnmouvement false))))))))

(event EventBeginPlay
  (bind _asbp_third_person_character (Utilities|Casting|CastToBP_ThirdPersonCharacter (Game|GetPlayerCharacter 0)))
  (Variables|Default|SetJoueru _asbp_third_person_character)
  (Variables|Default|SetPosdepart (Transformation|GetWorldLocation (Variables|Default|GetDefaultSceneRoot)))
  (Utilities|Time|SetTimerbyEvent (delegate Custom|CustomEvent) 0.1 true))

(fn ConstructionScript)