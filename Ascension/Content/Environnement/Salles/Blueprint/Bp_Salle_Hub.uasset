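; Hub room actor for the Ascension game that sets up its camera and entrance/exit pieces on BeginPlay.
; It caches GI_Ascension, then calls CameraSwitch with the SpawnCaméra location and spawns a BP_Ascenseur elevator at the SpawnDarriver marker.
; When the game instance's SallesRencontrésTotal count is zero, meaning no rooms encountered yet, it also spawns a BP_Mur wall at the SpawnDeDépart marker.
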(event EventBeginPlay
  (bind _spawn_d_arriver (Variables|Default|GetSpawn%20D'arriver))
  (bind _spawn_de_départ (Variables|Default|GetSpawn%20de%20départ))
  ;[1 0.3516 0] Références
  (bind _asgi_ascension (Utilities|Casting|CastToGI_Ascension (Game|GetGameInstance)))
  (Variables|Default|SetGI%20Ascension _asgi_ascension)
  (Utilities|FlowControl|Sequence
    (:then_0
      (CallFunction|CameraSwitch (Transformation|GetWorldLocation (Variables|Default|GetSpawn%20Caméra))))
    (:then_1
      (Game|SpawnActorfromClass "/Game/Environnement/Ascenseur/BP_Ascenseur.BP_Ascenseur_C" (Math|Transform|MakeTransform (Transformation|GetWorldLocation _spawn_d_arriver) (Transformation|GetWorldRotation _spawn_d_arriver) "1.000000,1.000000,1.000000") "Undefined" "MultiplyWithRoot" 0 0))
    (:then_2
      (if (== (Variables|/Game/GI_Ascension.GI_Ascension_C|GetSalles%20rencontrés%20total (Variables|Default|GetGI%20Ascension)) 0)
        (Game|SpawnActorfromClass "/Game/Environnement/Salles/Mur/BP_Mur.BP_Mur_C" (Math|Transform|MakeTransform (Transformation|GetWorldLocation _spawn_de_départ) (Transformation|GetWorldRotation _spawn_de_départ) "1.000000,1.000000,1.000000") "Undefined" "MultiplyWithRoot" 0 0)))))

(fn ConstructionScript)