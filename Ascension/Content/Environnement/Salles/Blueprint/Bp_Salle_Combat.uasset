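; Combat room actor that sets up its camera, two elevators and an enemy, reflecting whether the last fight was won.
; On BeginPlay it caches the game instance and player, switches the camera to its spawn point, then spawns ID-numbered elevators at left and right markers.
; Elevator walls start visible and solid.
; If GI_Ascension flags a won fight, it opens those walls, destroys the enemy component and resets the flag.
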(event EventBeginPlay
  (bind _id_spawn_ascenseur (Variables|Default|GetID_Spawn_Ascenseur))
  (Utilities|FlowControl|Sequence
    (:then_0
      ;[0.05469 0 1] Références
      (bind _asgi_ascension (Utilities|Casting|CastToGI_Ascension (Game|GetGameInstance)))
      (Variables|Default|SetGI%20Ascension _asgi_ascension)
      (bind _asbp_third_person_character (Utilities|Casting|CastToBP_ThirdPersonCharacter (Game|GetPlayerCharacter 0)))
      (Variables|Default|SetPlayer _asbp_third_person_character))
    (:then_1
      (Utilities|FlowControl|Sequence
        (:then_0
          (CallFunction|CameraSwitch (Transformation|GetWorldLocation (Variables|Default|GetSpawn%20Camera))))
        (:then_1
          (for _array_element (Utilities|Array|MakeArray (Variables|Default|GetSpawn_AscenseurGauche) (Variables|Default|GetSpawn_AscenseurDroite))
            (bind _returnvalue (Game|SpawnActorfromClass "/Game/Environnement/Ascenseur/BP_Ascenseur.BP_Ascenseur_C" (Math|Transform|MakeTransform (Transformation|GetWorldLocation _array_element) (Transformation|GetWorldRotation _array_element) "1.000000,1.000000,1.000000") "Undefined" "MultiplyWithRoot" 0 0))
            (Variables|/Game/Environnement/Ascenseur/BP_Ascenseur.BP_Ascenseur_C|SetID _returnvalue _id_spawn_ascenseur)
            (Math|Integer|IncrementInt _id_spawn_ascenseur
              (:%20%20
                (Rendering|SetVisibility (Variables|/Game/Environnement/Ascenseur/BP_Ascenseur.BP_Ascenseur_C|GetMur _returnvalue) true false)
                (Collision|SetCollisionEnabled (Variables|/Game/Environnement/Ascenseur/BP_Ascenseur.BP_Ascenseur_C|GetMur _returnvalue) "QueryAndPhysics")
                ;[0 1 0.4844] Si le combat à était gagné alors Retirer les "portes" fermés de l'ascenseur
                (if (Variables|/Game/GI_Ascension.GI_Ascension_C|GetDernier%20Combat%20Gagner%20? (Variables|Default|GetGI%20Ascension))
                  (Rendering|SetVisibility (Variables|/Game/Environnement/Ascenseur/BP_Ascenseur.BP_Ascenseur_C|GetMur _returnvalue) false false)
                  (Collision|SetCollisionEnabled (Variables|/Game/Environnement/Ascenseur/BP_Ascenseur.BP_Ascenseur_C|GetMur _returnvalue) "NoCollision")))))
          ;[0.9688 0 1] Si le combat à était gagner : Alors destruction de l'ennemi
          (if (Variables|/Game/GI_Ascension.GI_Ascension_C|GetDernier%20Combat%20Gagner%20? (Variables|Default|GetGI%20Ascension))
            (Components|DestroyComponent (Variables|Default|GetEnnemie))
            (Variables|/Game/GI_Ascension.GI_Ascension_C|SetDernier%20Combat%20Gagner%20? (Variables|Default|GetGI%20Ascension) false)))))))

(fn ConstructionScript)