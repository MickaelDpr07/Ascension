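; Two-way sliding double door between rooms that automatically walks the player character through.
; Entry or exit box overlap recenters the NavMeshBoundsVolume on the player, notifies navigation, disables input and slides both panels apart via timeline.
; SimpleMoveToLocation then sends the player to that side's target point.
; A looping timer, never cleared, polls arrival, then restores input and closes the door with a reversed timeline.
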(event OnComponentBeginOverlap(Boxentrer)
  (params (OverlappedComponent :type Primitive%20Component%20Object%20Reference) (OtherActor :type Actor%20Object%20Reference) (OtherComp :type Primitive%20Component%20Object%20Reference) (OtherBodyIndex :type Integer) (bFromSweep :type Boolean) (SweepResult :type Hit%20Result%20Structure%20%28by%20ref%29))
  (bind _returnvalue (Game|GetPlayerController 0))
  (if (not (Variables|Default|GetPorteenouverture))
    (Variables|Default|SetPorteenouverture true)
    (bind _returnvalue_2 (Actor|GetActorOfClass "/Script/NavigationSystem.NavMeshBoundsVolume"))
    (Transformation|SetActorLocation _returnvalue_2 (Transformation|GetActorLocation (Variables|Default|GetJoueur)) false false)
    (Class|NavigationSystemV1|OnNavigationBoundsUpdated (Class|NavigationSystemV1|GetNavigationSystem) _returnvalue_2)
    (Input|DisableInput (Pawn|GetControlledPawn _returnvalue) _returnvalue)
    (Variables|Default|SetPeut%20Prendre%20la%20Porte false)
    (bind _newtrack_0 (Timeline|portedroite PlayFromStart)
      (:Update
        (Transformation|SetRelativeLocation (Variables|Default|GetPorte%20droite) (Math|Vector|MakeVector (.x _newtrack_0) 0.0 56.350905) false false)
        (Transformation|SetRelativeLocation (Variables|Default|GetPorte%20gauche) (Math|Vector|MakeVector (* (.x _newtrack_0) -1.0) 0.0 56.350905) false false))
      (:Finished
        (AI|Navigation|SimpleMovetoLocation (Game|GetPlayerController (Variables|/Script/Engine.Pawn|GetPlayerState (Variables|Default|GetJoueur))) (Transformation|GetWorldLocation (Variables|Default|GetLocationDanssalle)))
        (Utilities|Time|SetTimerbyEvent (delegate Custom|At%20destination) 0.1 true)))))

(event OnComponentBeginOverlap(Boxsortie)
  (params (OverlappedComponent :type Primitive%20Component%20Object%20Reference) (OtherActor :type Actor%20Object%20Reference) (OtherComp :type Primitive%20Component%20Object%20Reference) (OtherBodyIndex :type Integer) (bFromSweep :type Boolean) (SweepResult :type Hit%20Result%20Structure%20%28by%20ref%29))
  (bind _returnvalue (Game|GetPlayerController 0))
  (if (not (Variables|Default|GetPorteenouverture))
    (Variables|Default|SetPorteenouverture true)
    (bind _returnvalue_2 (Actor|GetActorOfClass "/Script/NavigationSystem.NavMeshBoundsVolume"))
    (Transformation|SetActorLocation _returnvalue_2 (Transformation|GetActorLocation (Variables|Default|GetJoueur)) false false)
    (Class|NavigationSystemV1|OnNavigationBoundsUpdated (Class|NavigationSystemV1|GetNavigationSystem) _returnvalue_2)
    (Input|DisableInput (Pawn|GetControlledPawn _returnvalue) _returnvalue)
    (Variables|Default|SetPeut%20Prendre%20la%20Porte false)
    (bind _newtrack_0 (Timeline|Timeline_2 PlayFromStart)
      (:Update
        (Transformation|SetRelativeLocation (Variables|Default|GetPorte%20droite) (Math|Vector|MakeVector (.x _newtrack_0) 0.0 56.350905) false false)
        (Transformation|SetRelativeLocation (Variables|Default|GetPorte%20gauche) (Math|Vector|MakeVector (* (.x _newtrack_0) -1.0) 0.0 56.350905) false false))
      (:Finished
        (AI|Navigation|SimpleMovetoLocation (Game|GetPlayerController (Variables|/Script/Engine.Pawn|GetPlayerState (Variables|Default|GetJoueur))) (Transformation|GetWorldLocation (Variables|Default|GetLocationretour)))
        (Utilities|Time|SetTimerbyEvent (delegate Custom|CustomEvent) 0.1 true)))))

(event Custom|CustomEvent
  (bind _returnvalue (Game|GetPlayerController 0))
  (if (Utilities|Operators|EqualEqual (Transformation|GetWorldLocation (Variables|/Script/Engine.Character|GetMesh (Variables|Default|GetJoueur))) (Transformation|GetWorldLocation (Variables|Default|GetLocationretour)) 5e+01)
    (if (not (Variables|Default|GetPeut%20Prendre%20la%20Porte))
      (Variables|Default|SetPeut%20Prendre%20la%20Porte true)
      (Input|EnableInput (Pawn|GetControlledPawn _returnvalue) _returnvalue)
      (bind _newtrack_0 (Timeline|Timeline_4 ReverseFromEnd)
        (:Update
          (Transformation|SetRelativeLocation (Variables|Default|GetPorte%20droite) (Math|Vector|MakeVector (.x _newtrack_0) 0.0 56.350905) false false)
          (Transformation|SetRelativeLocation (Variables|Default|GetPorte%20gauche) (Math|Vector|MakeVector (* (.x _newtrack_0) -1.0) 0.0 56.350905) false false))
        (:Finished
          (Variables|Default|SetPorteenouverture false))))))

(event Custom|At%20destination
  (bind _returnvalue (Game|GetPlayerController 0))
  (if (Utilities|Operators|EqualEqual (Transformation|GetWorldLocation (Variables|/Script/Engine.Character|GetMesh (Variables|Default|GetJoueur))) (Transformation|GetWorldLocation (Variables|Default|GetLocationDanssalle)) 5e+01)
    (if (not (Variables|Default|GetPeut%20Prendre%20la%20Porte))
      (Variables|Default|SetPeut%20Prendre%20la%20Porte true)
      (Input|EnableInput (Pawn|GetControlledPawn _returnvalue) _returnvalue)
      (bind _newtrack_0 (Timeline|Timeline_0 ReverseFromEnd)
        (:Update
          (Transformation|SetRelativeLocation (Variables|Default|GetPorte%20droite) (Math|Vector|MakeVector (.x _newtrack_0) 0.0 56.350905) false false)
          (Transformation|SetRelativeLocation (Variables|Default|GetPorte%20gauche) (Math|Vector|MakeVector (* (.x _newtrack_0) -1.0) 0.0 56.350905) false false))
        (:Finished
          (Variables|Default|SetPorteenouverture false))))))

(event EventBeginPlay
  (bind _returnvalue (Actor|GetActorOfClass "/Game/ThirdPerson/Blueprints/BP_ThirdPersonCharacter.BP_ThirdPersonCharacter_C"))
  (Variables|Default|SetJoueur _returnvalue))

(fn ConstructionScript)