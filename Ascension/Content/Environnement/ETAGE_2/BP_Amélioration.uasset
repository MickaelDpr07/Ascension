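; BP_Amélioration is a trigger actor that opens the competence (skill) upgrade screen when the player walks into it.
; On BeginPlay it caches the player as BP_ThirdPersonCharacter.
; When that character begins overlapping the Box, it creates a new Widget_Competence, adds it to the viewport and sets the movement mode to None to freeze the player.
; Nothing in this Blueprint removes the widget or restores movement.
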(event OnComponentBeginOverlap(Box)
  (params (OverlappedComponent :type Primitive%20Component%20Object%20Reference) (OtherActor :type Actor%20Object%20Reference) (OtherComp :type Primitive%20Component%20Object%20Reference) (OtherBodyIndex :type Integer) (bFromSweep :type Boolean) (SweepResult :type Hit%20Result%20Structure%20%28by%20ref%29))
  (if (== OtherActor (Variables|Default|GetPlayer))
    (bind _returnvalue (UserInterface|CreateWidget "/Game/ThirdPerson/Blueprints/Amélioration/Widget_Competence.Widget_Competence_C"))
    (UserInterface|Viewport|AddtoViewport _returnvalue 0)
    (Pawn|Components|CharacterMovement|SetMovementMode (Variables|/Script/Engine.Character|GetCharacterMovement (Variables|Default|GetPlayer)) "MOVE_None" 0)))

(event EventBeginPlay
  (bind _asbp_third_person_character (Utilities|Casting|CastToBP_ThirdPersonCharacter (Game|GetPlayerCharacter 0)))
  (Variables|Default|SetPlayer _asbp_third_person_character))

(fn ConstructionScript)