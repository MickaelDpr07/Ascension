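; Elevator actor that carries the player up to the next room, offering a room type on its text label.
; On first player overlap, it closes a wall, rises, destroys the previous room and other elevators, then spawns its choice.
; GI_Ascension's desired-versus-actual room percentages steer offers: elevator 0 takes the most under-represented, elevator 1 a random pick from a trimmed list.
; A room counter periodically forces all-HUB offers, preceded by all-combat offers.
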(event OnComponentBeginOverlap(Box)
  (params (OverlappedComponent :type Primitive%20Component%20Object%20Reference) (OtherActor :type Actor%20Object%20Reference) (OtherComp :type Primitive%20Component%20Object%20Reference) (OtherBodyIndex :type Integer) (bFromSweep :type Boolean) (SweepResult :type Hit%20Result%20Structure%20%28by%20ref%29))
  (bind _gi_ascension (Variables|Default|GetGI%20Ascension))
  (bind _spawn (Variables|Default|GetSpawn))
  (bind _mur (Variables|Default|GetMur))
  (bind _mur_2 (Variables|Default|GetMur))
  (bind _defaultsceneroot (Variables|Default|GetDefaultSceneRoot))
  (bind _gi_ascension_2 (Variables|Default|GetGI%20Ascension))
  (bind _returnvalue (Transformation|GetWorldLocation _spawn))
  (bind _returnvalue_2 (Transformation|GetWorldLocation _defaultsceneroot))
  (if (== OtherActor (Variables|Default|GetPlayer))
    (Utilities|FlowControl|DoOnce false
      (:Completed
        (Rendering|SetVisibility _mur_2 true false)
        (Collision|SetCollisionEnabled _mur_2 "QueryAndPhysics")
        ;[1 0 0.2109] Mouvement Ascenseur
        (Timeline|Ascenseur_Movement PlayFromStart
          (:Update
            (Transformation|SetActorLocation (Math|Vector|MakeVector (.x _returnvalue_2) (.y _returnvalue_2) (+ (.z _returnvalue_2) 1e+01)) false false))
          (:Finished
            (Rendering|SetVisibility _mur false false)
            (Collision|SetCollisionEnabled _mur "NoCollision")
            ;[1 0.9141 0] Spawn salle parmis les deux proposés
            (Actor|DestroyActor (Variables|/Game/GI_Ascension.GI_Ascension_C|GetDerniereSalle (Variables|Default|GetGI%20Ascension)))
            (Variables|Default|SetFutur_Spawn (Utilities|Select :Index (Variables|Default|GetID) :Option%200 (Variables|Default|GetChoix1) :Option%201 (Variables|Default|GetChoix2)))
            ;;[0 1 0.7891] Suppression Anciens Ascenseur et Changement Index Actuel
            (bind _outactors (Actor|GetAllActorsOfClass "BP_Ascenseur_C"))
            (for _array_element _outactors
              (if (!= (Variables|BP_Ascenseur_C|GetID _array_element) (Variables|Default|GetID))
                (Actor|DestroyActor _array_element)))
            (Variables|Default|SetID 2)
            (bind _returnvalue_3 (Game|SpawnActorfromClass (Variables|Default|GetFutur_Spawn) (Math|Transform|MakeTransform (Math|Vector|MakeVector (.x _returnvalue) (.y _returnvalue) (.z _returnvalue)) (Transformation|GetWorldRotation _spawn) "1.000000,1.000000,1.000000") "Undefined" "MultiplyWithRoot" 0 0))
            (bind _output_get (Variables|/Game/GI_Ascension.GI_Ascension_C|SetDerniereSalle _gi_ascension_2 _returnvalue_3))
            ;[0 1 0.3438] Si la salle qui spawn est égale à un élément de la liste du gm alors lui ajout +1
            (bind _keys (Utilities|Map|Keys (Variables|/Game/GI_Ascension.GI_Ascension_C|GetSalles%20rencontrés _gi_ascension_2)))
            (for _array_element_2 _keys
              (if (== _array_element_2 _output_get)
                (Utilities|Map|Add (Variables|/Game/GI_Ascension.GI_Ascension_C|GetSalles%20rencontrés (Variables|Default|GetGI%20Ascension)) _array_element_2 (+ (.Value (Utilities|Map|Find (Variables|/Game/GI_Ascension.GI_Ascension_C|GetSalles%20rencontrés (Variables|Default|GetGI%20Ascension)) _array_element_2)) 1.0))
                ;[0.6641 1 0] Ajout +1 au nombres de salles rencontrés
                (Variables|/Game/GI_Ascension.GI_Ascension_C|SetSalles%20rencontrés%20total _gi_ascension (+ (Variables|/Game/GI_Ascension.GI_Ascension_C|GetSalles%20rencontrés%20total _gi_ascension) 1))))
            (CallFunction|PourcentageSallesRencontrés)
            (CallFunction|DifférenceSouhaitéEtRéel)
            (CallFunction|EvenementsSalles)))))))

(event EventBeginPlay
  (Utilities|FlowControl|Delay 0.1)
  (bind _asgi_ascension (Utilities|Casting|CastToGI_Ascension (Game|GetGameInstance)))
  (Variables|Default|SetGI%20Ascension _asgi_ascension)
  (bind _asbp_third_person_character (Utilities|Casting|CastToBP_ThirdPersonCharacter (Game|GetPlayerCharacter 0)))
  (Variables|Default|SetPlayer _asbp_third_person_character)
  (CallFunction|EvenementsSalles))

(fn ConstructionScript)

(fn ChoixLePlusEloigné
  ;[0 1 0.1328] Séléction de la salle la plus éloigné du pourcentage souhaité
  (Variables|1erChoix|SetIndex%20le%20plus%20éloigner 0)
  (Variables|1erchoix|SetValeur%20Plus%20Eloigne 0.0)
  (for (_array_element _array_index) (Variables|/Game/GI_Ascension.GI_Ascension_C|GetDifférences%20souhaité/réel (Variables|Default|GetGI%20Ascension))
    (if (> _array_element (Variables|1erchoix|GetValeur%20Plus%20Eloigne))
      (Variables|1erchoix|SetValeur%20Plus%20Eloigne _array_element)
      (Variables|1erChoix|SetIndex%20le%20plus%20éloigner _array_index))))

(fn ChoixDes3PlusÉloignés
  (bind _gi_ascension (Variables|Default|GetGI%20Ascension))
  ;[0.3359 0 1] Copie de la liste de salles dans un array et suppression de l'élément le plus proche de 0
  (bind _keys (Utilities|Map|Keys (Variables|/Game/GI_Ascension.GI_Ascension_C|GetListSalles/PourcentageSouhaité _gi_ascension)))
  (bind _output_get (Variables|deuxièmechoix|SetListe2èmeChoix _keys))
  (for (_ _array_index) _output_get
    (if (== _array_index (.IndexOfMinValue (Math|Float|MinOfFloatArray (Variables|/Game/GI_Ascension.GI_Ascension_C|GetDifférences%20souhaité/réel _gi_ascension))))
      (Utilities|Array|RemoveIndex (Variables|deuxièmechoix|GetListe2èmeChoix) _array_index))))

(fn PourcentageSallesRencontrés
  (bind _gi_ascension (Variables|Default|GetGI%20Ascension))
  ;[1 0 0.2344] Pourcentage des salles rencontrés
  (bind _values (Utilities|Map|Values (Variables|/Game/GI_Ascension.GI_Ascension_C|GetSalles%20rencontrés _gi_ascension)))
  (for (_array_element _array_index) _values
    (Utilities|Array|SetArrayElem (Variables|/Game/GI_Ascension.GI_Ascension_C|GetListSalles/PourcentageRéel _gi_ascension) _array_index (/ _array_element (Variables|/Game/GI_Ascension.GI_Ascension_C|GetSalles%20rencontrés%20total _gi_ascension)))))

(fn DifférenceSouhaitéEtRéel
  (bind _gi_ascension (Variables|Default|GetGI%20Ascension))
  ;[0.9688 0 1] Calcul de la différence entre le pourcentage souhaité et le pourcentage réel
  (bind _values (Utilities|Map|Values (Variables|/Game/GI_Ascension.GI_Ascension_C|GetListSalles/PourcentageSouhaité _gi_ascension)))
  (for (_ _array_index) _values
    (bind _output_get (Variables|Default|SetArray%20Index _array_index))
    (Utilities|Array|SetArrayElem (Variables|/Game/GI_Ascension.GI_Ascension_C|GetDifférences%20souhaité/réel (Variables|Default|GetGI%20Ascension)) _output_get (- (Utilities|Array|Get(acopy) _values (Variables|Default|GetArray%20Index)) (Utilities|Array|Get(acopy) (Variables|/Game/GI_Ascension.GI_Ascension_C|GetListSalles/PourcentageRéel _gi_ascension) (Variables|Default|GetArray%20Index))))))

(fn EvenementsSalles
  (bind _gi_ascension (Variables|Default|GetGI%20Ascension))
  (bind _gi_ascension_2 (Variables|Default|GetGI%20Ascension))
  (bind _liste2èmechoix (Variables|deuxièmechoix|GetListe2èmeChoix))
  (switch int (- (Variables|/Game/GI_Ascension.GI_Ascension_C|GetSalles%20rencontrés%20total _gi_ascension) (Variables|/Game/GI_Ascension.GI_Ascension_C|GetProchaineSalleHUB _gi_ascension))
    (:Default
      ;[1 0.4219 0] Proposition de salle en fonction de l'ascenseur
      (switch int (Variables|Default|GetID)
        (:0
          (Development|PrintString "0")
          ;[0 1 0.01562] Choisi la salle la plus éloigné de 0
          (CallFunction|ChoixLePlusEloigné)
          (bind _keys (Utilities|Map|Keys (Variables|/Game/GI_Ascension.GI_Ascension_C|GetListSalles/PourcentageSouhaité (Variables|Default|GetGI%20Ascension))))
          (bind _outactors (Actor|GetAllActorsOfClass "BP_Ascenseur_C"))
          (for _array_element _outactors
            (if (== (Variables|BP_Ascenseur_C|GetID _array_element) (Variables|Default|GetID))
              (bind _output_get (Variables|Default|SetChoix1 (Utilities|Array|Get(acopy) _keys (Variables|1erChoix|GetIndex%20le%20plus%20éloigner))))
              (Rendering|Components|TextRender|SetText (Variables|BP_Ascenseur_C|GetTxt_Choix _array_element) (Utilities|Text|ToText(String) (Utilities|GetClassDisplayName _output_get))))))
        (:1
          (Development|PrintString "1")
          ;[0.1719 1 0] Choisir un élément au hasard parmis les plus éloignés
          (CallFunction|ChoixDes3PlusÉloignés)
          (bind _outactors_2 (Actor|GetAllActorsOfClass "BP_Ascenseur_C"))
          (for _array_element_2 _outactors_2
            (if (== (Variables|BP_Ascenseur_C|GetID _array_element_2) (Variables|Default|GetID))
              (bind _output_get_2 (Variables|Default|SetChoix2 (Utilities|Array|Get(acopy) _liste2èmechoix (Math|Random|RandomInteger (Utilities|Array|Length _liste2èmechoix)))))
              (Rendering|Components|TextRender|SetText (Variables|BP_Ascenseur_C|GetTxt_Choix _array_element_2) (Utilities|Text|ToText(String) (Utilities|GetClassDisplayName _output_get_2))))))))
    (:-1
      ;[1 0.2578 0] Les salles proposés ne sont que des Combats
      (bind _keys_2 (Utilities|Map|Keys (Variables|/Game/GI_Ascension.GI_Ascension_C|GetListSalles/PourcentageSouhaité (Variables|Default|GetGI%20Ascension))))
      (bind _outactors_3 (Actor|GetAllActorsOfClass "BP_Ascenseur_C"))
      (for _array_element_3 _outactors_3
        (Variables|BP_Ascenseur_C|SetChoix1 _array_element_3 (Utilities|Array|Get(acopy) _keys_2))
        (Variables|BP_Ascenseur_C|SetChoix2 _array_element_3 (Utilities|Array|Get(acopy) _keys_2))
        (Rendering|Components|TextRender|SetText (Variables|BP_Ascenseur_C|GetTxt_Choix _array_element_3) (Utilities|Text|ToText(String) (Utilities|GetClassDisplayName (Utilities|Array|Get(acopy) _keys_2))))))
    (:0
      ;[0.9219 1 0] Les salles proposés ne sont que des HUBS
      (Variables|/Game/GI_Ascension.GI_Ascension_C|SetProchaineSalleHUB _gi_ascension_2 (+ (Variables|/Game/GI_Ascension.GI_Ascension_C|GetProchaineSalleHUB _gi_ascension_2) 10))
      (bind _keys_3 (Utilities|Map|Keys (Variables|/Game/GI_Ascension.GI_Ascension_C|GetListSalles/PourcentageSouhaité _gi_ascension_2)))
      (bind _outactors_4 (Actor|GetAllActorsOfClass "BP_Ascenseur_C"))
      (for _array_element_4 _outactors_4
        (Variables|BP_Ascenseur_C|SetChoix1 _array_element_4 (Utilities|Array|Get(acopy) _keys_3 3))
        (Variables|BP_Ascenseur_C|SetChoix2 _array_element_4 (Utilities|Array|Get(acopy) _keys_3 3))
        (Rendering|Components|TextRender|SetText (Variables|BP_Ascenseur_C|GetTxt_Choix _array_element_4) (Utilities|Text|ToText(String) (Utilities|GetClassDisplayName (Utilities|Array|Get(acopy) _keys_3 3))))))))