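; Trigger actor that changes the level's exponential height fog density when the player walks into one of its two volumes.
; On BeginPlay it caches the third-person player character and the first ExponentialHeightFog actor found.
; Overlapping Activated sets density to 1.0, while overlapping Disable applies a timeline track's current value.
; Neither timeline is ever played, so both changes are instant rather than animated fades.
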(event OnComponentBeginOverlap(Disable)
  (params (OverlappedComponent :type Primitive%20Component%20Object%20Reference) (OtherActor :type Actor%20Object%20Reference) (OtherComp :type Primitive%20Component%20Object%20Reference) (OtherBodyIndex :type Integer) (bFromSweep :type Boolean) (SweepResult :type Hit%20Result%20Structure%20%28by%20ref%29))
  (if (== OtherActor (Variables|Default|GetPlayer))
    (Class|ExponentialHeightFogComponent|SetFogDensity (Variables|/Script/Engine.ExponentialHeightFog|GetComponent (Variables|Default|GetFog)) (stale _newtrack_0))))

(event OnComponentBeginOverlap(Activated)
  (params (OverlappedComponent :type Primitive%20Component%20Object%20Reference) (OtherActor :type Actor%20Object%20Reference) (OtherComp :type Primitive%20Component%20Object%20Reference) (OtherBodyIndex :type Integer) (bFromSweep :type Boolean) (SweepResult :type Hit%20Result%20Structure%20%28by%20ref%29))
  (if (== OtherActor (Variables|Default|GetPlayer))
    (Class|ExponentialHeightFogComponent|SetFogDensity (Variables|/Script/Engine.ExponentialHeightFog|GetComponent (Variables|Default|GetFog)) 1.0)))

(event Custom|CustomEvent
  (params (OverlappedComponent :type Primitive%20Component%20Object%20Reference) (OtherActor :type Actor%20Object%20Reference) (OtherComp :type Primitive%20Component%20Object%20Reference) (OtherBodyIndex :type Integer) (bFromSweep :type Boolean) (SweepResult :type Hit%20Result%20Structure%20%28by%20ref%29)))

(event EventBeginPlay
  (bind _asbp_third_person_character (Utilities|Casting|CastToBP_ThirdPersonCharacter (Game|GetPlayerCharacter 0)))
  (Variables|Default|SetPlayer _asbp_third_person_character)
  (bind _returnvalue (Actor|GetActorOfClass "/Script/Engine.ExponentialHeightFog"))
  (Variables|Default|SetFog _returnvalue))

(fn ConstructionScript)