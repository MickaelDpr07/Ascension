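; Accreditation checkpoint: a hologram barrier that lets the player through only with a high enough Accreditation, with the required level shown as text.
; On box overlap, it compares the player's Accreditation to the requirement, toggles barrier collision and recolours hologram and camera through dynamic materials.
; The camera pivot tracks the player on Tick while inside.
; On exit, the pivot returns to its initial rotation and colours change, but collision is left as set.
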(event OnComponentBeginOverlap(Box)
  (params (OverlappedComponent :type Primitive%20Component%20Object%20Reference) (OtherActor :type Actor%20Object%20Reference) (OtherComp :type Primitive%20Component%20Object%20Reference) (OtherBodyIndex :type Integer) (bFromSweep :type Boolean) (SweepResult :type Hit%20Result%20Structure%20%28by%20ref%29))
  (bind _color (Variables|Default|GetColor))
  (bind _color_2 (Variables|Default|GetColor))
  (bind _pivotcamera (Variables|Default|GetPivotCamera))
  (bind _output (Utilities|Array|Get(acopy) _color_2 2))
  (bind _output_2 (Utilities|Array|Get(acopy) _color 1))
  (bind _asbp_third_person_character (Utilities|Casting|CastToBP_ThirdPersonCharacter OtherActor))
  (bind _output_get (Variables|Default|SetAs%20BP%20Third%20Person%20Character _asbp_third_person_character))
  (Components|MoveComponentTo _pivotcamera (Variables|/Script/Engine.SceneComponent|GetRelativeLocation _pivotcamera) (Math|Rotator|MakeRotator (.roll (Math|Rotator|FindLookatRotation (Transformation|GetWorldLocation _pivotcamera) (Transformation|GetActorLocation _asbp_third_person_character))) (.pitch (Math|Rotator|FindLookatRotation (Transformation|GetWorldLocation _pivotcamera) (Transformation|GetActorLocation _asbp_third_person_character))) (.yaw (Math|Rotator|FindLookatRotation (Transformation|GetWorldLocation _pivotcamera) (Transformation|GetActorLocation _asbp_third_person_character)))) false false 0.2 false)
  (Variables|Default|SetPlayerInBox true)
  (if (>= (Variables|/Game/ThirdPerson/Blueprints/BP_ThirdPersonCharacter.BP_ThirdPersonCharacter_C|GetAccreditation _output_get) (Variables|Default|GetAccréditationNécessaire))
    (Utilities|FlowControl|Sequence
      (:then_0
        (Collision|SetCollisionEnabled (Variables|Default|GetTest) "NoCollision"))
      (:then_1
        (Rendering|Material|SetVectorParameterValue (Variables|Default|GetMaterialInstance) "Color" _output :!class /Script/Engine.MaterialInstanceDynamic))
      (:then_2
        (Rendering|Material|SetVectorParameterValue (Variables|Default|GetMaterialCamera) "Couleur" _output :!class /Script/Engine.MaterialInstanceDynamic)))
    (else
      (Utilities|FlowControl|Sequence
        (:then_0
          (Rendering|Material|SetVectorParameterValue (Variables|Default|GetMaterialInstance) "Color" _output_2 :!class /Script/Engine.MaterialInstanceDynamic))
        (:then_1
          (Rendering|Material|SetVectorParameterValue (Variables|Default|GetMaterialCamera) "Couleur" _output_2 :!class /Script/Engine.MaterialInstanceDynamic))
        (:then_2
          (Collision|SetCollisionEnabled (Variables|Default|GetTest) "QueryAndPhysics"))))))

(event OnComponentEndOverlap(Box)
  (params (OverlappedComponent :type Primitive%20Component%20Object%20Reference) (OtherActor :type Actor%20Object%20Reference) (OtherComp :type Primitive%20Component%20Object%20Reference) (OtherBodyIndex :type Integer))
  (bind _pivotcamera (Variables|Default|GetPivotCamera))
  (bind _asbp_third_person_character (Utilities|Casting|CastToBP_ThirdPersonCharacter OtherActor))
  (Variables|Default|SetAs%20BP%20Third%20Person%20Character _asbp_third_person_character)
  (Variables|Default|SetPlayerInBox false)
  (Components|MoveComponentTo _pivotcamera (Variables|/Script/Engine.SceneComponent|GetRelativeLocation _pivotcamera) (Variables|Default|GetRelative%20Rotation) false false 0.2 false)
  (Rendering|Material|SetVectorParameterValue (Variables|Default|GetMaterialCamera) "Couleur" (Utilities|Array|Get(acopy) (Variables|Default|GetColor) 2) :!class /Script/Engine.MaterialInstanceDynamic)
  (Rendering|Material|SetVectorParameterValue (Variables|Default|GetMaterialInstance) "Color" (Utilities|Array|Get(acopy) (Variables|Default|GetColor)) :!class /Script/Engine.MaterialInstanceDynamic))

(event EventBeginPlay
  (bind _color (Variables|Default|GetColor))
  (bind _output (Utilities|Array|Get(acopy) _color))
  (Utilities|FlowControl|Sequence
    (:then_0
      (bind _returnvalue (Rendering|Material|CreateDynamicMaterialInstance (Variables|Default|GetTest) 0 "/Game/Material/Hologram/M_Hologram.M_Hologram" "None" :!class /Script/Engine.PrimitiveComponent))
      (bind _output_get (Variables|Default|SetMaterialInstance _returnvalue))
      (Rendering|Material|SetVectorParameterValue _returnvalue "Color" _output :!class /Script/Engine.MaterialInstanceDynamic)
      (Variables|Default|SetRelative%20Rotation (Variables|/Script/Engine.SceneComponent|GetRelativeRotation (Variables|Default|GetPivotCamera))))
    (:then_1
      (bind _returnvalue_2 (Rendering|Material|CreateDynamicMaterialInstance (Variables|Default|GetCouleur_Camera) 0 "/Game/Environnement/Bp_TestAccréditation/Material/M_Couleur_Camera.M_Couleur_Camera" "None" :!class /Script/Engine.PrimitiveComponent))
      (bind _output_get_2 (Variables|Default|SetMaterialCamera _returnvalue_2))
      (Rendering|Material|SetVectorParameterValue _output_get_2 "Couleur" _output :!class /Script/Engine.MaterialInstanceDynamic))))

(event EventTick
  (params (DeltaSeconds :type Float%20%28single-precision%29))
  (bind _pivotcamera (Variables|Default|GetPivotCamera))
  (bind _as_bp_third_person_character (Variables|Default|GetAs%20BP%20Third%20Person%20Character))
  (bind _returnvalue (Transformation|GetWorldLocation _pivotcamera))
  (bind _returnvalue_2 (Transformation|GetActorLocation _as_bp_third_person_character))
  (bind _returnvalue_3 (Math|Rotator|FindLookatRotation _returnvalue _returnvalue_2))
  (if (Variables|Default|GetPlayerInBox)
    (Transformation|SetWorldRotation (Variables|Default|GetPivotCamera) (Math|Rotator|MakeRotator 0.0 (.pitch _returnvalue_3) (.yaw _returnvalue_3)) true false)))

(fn ConstructionScript
  (Rendering|Components|TextRender|SetText (Variables|Default|GetNuméroAccréditationNécessaire) (Utilities|Text|ToText(Integer) (Variables|Default|GetAccréditationNécessaire))))