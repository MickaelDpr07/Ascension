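; BP_Amelioration is an environment trigger that opens the skill (competence) screen when the player walks into it.
; BeginPlay caches the third-person character and the GM_Exploration game mode.
; When that character overlaps the Box, it creates and shows WB_Competence, then sets movement mode to None to freeze the player.
; It also sets WidgetSpecialOpen on the game mode to prevent stacked widgets; nothing here reverses either change.
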(event OnComponentBeginOverlap(Box)
  (params (OverlappedComponent :type Primitive%20Component%20Object%20Reference) (OtherActor :type Actor%20Object%20Reference) (OtherComp :type Primitive%20Component%20Object%20Reference) (OtherBodyIndex :type Integer) (bFromSweep :type Boolean) (SweepResult :type Hit%20Result%20Structure%20%28by%20ref%29))
  ;[0 0.5312 1] Test si c'est le joueur
  (if (== OtherActor (Variables|Default|GetPlayer))
    (bind _returnvalue (UserInterface|CreateWidget "/Game/ThirdPerson/Blueprints/Amélioration/WB_Competence.WB_Competence_C"))
    (UserInterface|Viewport|AddtoViewport _returnvalue 0)
    (Pawn|Components|CharacterMovement|SetMovementMode (Variables|/Script/Engine.Character|GetCharacterMovement (Variables|Default|GetPlayer)) "MOVE_None" 0)
    ;[0.7344 0 1] Empecher la superposition de widgets
    (Variables|/Game/GM_Exploration.GM_Exploration_C|SetWidget%20Special%20Open%20? (Variables|Default|GetGM%20Exploration) true)))

(event EventBeginPlay
  ;[0.9922 0 1] Références
  (bind _asbp_third_person_character (Utilities|Casting|CastToBP_ThirdPersonCharacter (Game|GetPlayerCharacter 0)))
  (Variables|Default|SetPlayer _asbp_third_person_character)
  (bind _asgm_exploration (Utilities|Casting|CastToGM_Exploration (Game|GetGameMode)))
  (Variables|Default|SetGM%20Exploration _asgm_exploration))

(fn ConstructionScript)