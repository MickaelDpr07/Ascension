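; Elevator offering the player's next room in a room-by-room ascent.
; On overlap it rises behind a temporary wall, replaces the previous room and other elevators with the chosen room, moves the navmesh bounds and auto-walks the player out.
; GameInstance tallies steer offers: one elevator shows the room type furthest below its target share, the other a random pick excluding both extremes.
; Combat and hub rooms are forced periodically; ten rooms trigger the end screen.
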(event OnComponentBeginOverlap(Box)
  (params (OverlappedComponent :type Primitive%20Component%20Object%20Reference) (OtherActor :type Actor%20Object%20Reference) (OtherComp :type Primitive%20Component%20Object%20Reference) (OtherBodyIndex :type Integer) (bFromSweep :type Boolean) (SweepResult :type Hit%20Result%20Structure%20%28by%20ref%29))
  (bind _gi_ascension (Variables|Default|GetGI%20Ascension))
  (bind _spawn (Variables|Default|GetSpawn))
  (bind _mur (Variables|Default|GetMur))
  (bind _gi_ascension_2 (Variables|Default|GetGI%20Ascension))
  (bind _mur_2 (Variables|Default|GetMur))
  (bind _defaultsceneroot (Variables|Default|GetDefaultSceneRoot))
  (bind _gi_ascension_3 (Variables|Default|GetGI%20Ascension))
  (bind _returnvalue (Transformation|GetWorldLocation _spawn))
  (bind _returnvalue_2 (Transformation|GetWorldLocation _defaultsceneroot))
  (if (== OtherActor (Variables|Default|GetPlayer))
    (Utilities|FlowControl|Sequence
      (:then_0
        (Utilities|FlowControl|DoOnce false
          (:Completed
            (Rendering|SetVisibility _mur_2 true false)
            (Collision|SetCollisionEnabled _mur_2 "QueryAndPhysics")
            ;[1 0 0.2109] Mouvement Ascenseur
            (Timeline|Ascenseur_Movement PlayFromStart
              (:Update
                (Transformation|SetActorLocation (Math|Vector|MakeVector (.x _returnvalue_2) (.y _returnvalue_2) (+ (.z _returnvalue_2) 1e+01)) false false))
              (:Finished
                ;[0 0.03906 1] Disparition du mur
                (Rendering|SetVisibility _mur false false)
                (Collision|SetCollisionEnabled _mur "NoCollision")
                ;[1 0.9141 0] Spawn salle parmis les deux proposés
                (Utilities|FlowControl|Sequence
                  (:then_0
                    (Utilities|FlowControl|Sequence
                      (:then_0
                        ;[0.5234 1 0] Destroy l'ancienne salle au début en supprimant le Hub Rez de Chaussé
                        (bind _returnvalue_3 (Actor|GetActorOfClass "/Game/Environnement/Salles/Blueprint/Bp_Salle_Hub.Bp_Salle_Hub_C"))
                        (Utilities|IsValid _returnvalue_3
                          (:Is%20Valid
                            (Actor|DestroyActor _returnvalue_3))))
                      (:then_1
                        ;[1 0 0.2812] Test la validité de la salle avant de la détruire (Correction premier lancement)
                        (Utilities|IsValid (Variables|/Game/GI_Ascension.GI_Ascension_C|GetDerniereSalle (Variables|Default|GetGI%20Ascension))
                          (:Is%20Valid
                            (Actor|DestroyActor (Variables|/Game/GI_Ascension.GI_Ascension_C|GetDerniereSalle (Variables|Default|GetGI%20Ascension))))))))
                  (:then_1
                    (Variables|Default|SetFutur_Spawn (Utilities|Select :Index (Variables|Default|GetID) :Option%200 (Variables|/Game/GI_Ascension.GI_Ascension_C|GetChoice1 _gi_ascension_2) :Option%201 (Variables|/Game/GI_Ascension.GI_Ascension_C|GetChoice2 _gi_ascension_2)))
                    ;;[0 1 0.7891] Suppression Anciens Ascenseur et Changement Index Actuel
                    (bind _outactors (Actor|GetAllActorsOfClass "BP_Ascenseur_C"))
                    (for _array_element _outactors
                      (if (!= (Variables|BP_Ascenseur_C|GetID _array_element) (Variables|Default|GetID))
                        (Utilities|IsValid _array_element
                          (:Is%20Valid
                            (Actor|DestroyActor _array_element)))))
                    (Variables|Default|SetID 2)
                    (Utilities|FlowControl|Sequence
                      (:then_0
                        ;[0.6641 1 0] Ajout +1 au nombres de salles rencontrés
                        (Variables|/Game/GI_Ascension.GI_Ascension_C|SetSalles%20rencontrés%20total _gi_ascension (+ (Variables|/Game/GI_Ascension.GI_Ascension_C|GetSalles%20rencontrés%20total _gi_ascension) 1)))
                      (:then_1
                        (bind _returnvalue_4 (Game|SpawnActorfromClass (Variables|Default|GetFutur_Spawn) (Math|Transform|MakeTransform (Math|Vector|MakeVector (.x _returnvalue) (.y _returnvalue) (.z _returnvalue)) (Transformation|GetWorldRotation _spawn) "1.000000,1.000000,1.000000") "Undefined" "MultiplyWithRoot" 0 0))
                        ;[1 0.3516 0] SET Dernière salle et sauvegarde de son type dans le GI
                        (bind _output_get (Variables|/Game/GI_Ascension.GI_Ascension_C|SetDerniereSalle (Variables|Default|GetGI%20Ascension) _returnvalue_4))
                        (Variables|/Game/GI_Ascension.GI_Ascension_C|SetPosition/Type%20Last%20Salle (Variables|Default|GetGI%20Ascension) (Utilities|Map|MakeMap (Utilities|GetClass _output_get) (Transformation|GetWorldTransform (Variables|Default|GetSpawn))))
                        (Utilities|FlowControl|Sequence
                          (:then_0
                            (Input|SetInputModeUIOnly (Game|GetPlayerController 0) 0 "DoNotLock" false)
                            (bind _returnvalue_5 (Actor|GetActorOfClass "/Script/NavigationSystem.NavMeshBoundsVolume"))
                            (Transformation|SetActorLocation _returnvalue_5 (Transformation|GetWorldLocation (Variables|/Script/Engine.Character|GetMesh (Variables|Default|GetPlayer))) false false)
                            ;[0.7109 1 0] Met à jour le navmesh
                            (Class|NavigationSystemV1|OnNavigationBoundsUpdated (Class|NavigationSystemV1|GetNavigationSystem) _returnvalue_5)
                            (Utilities|FlowControl|Delay 0.2)
                            (AI|Navigation|SimpleMovetoLocation (Game|GetPlayerController (Variables|/Script/Engine.Pawn|GetPlayerState (Variables|Default|GetPlayer))) (Transformation|GetWorldLocation (Variables|Default|GetDestination)))
                            (Utilities|Time|SetTimerbyEvent (delegate Custom|At%20destination) 0.1 true))
                          (:then_1
                            ;[0 1 0.3438] Si la salle qui spawn est égale à un élément de la liste du gm alors lui ajout +1
                            (bind _keys (Utilities|Map|Keys (Variables|/Game/GI_Ascension.GI_Ascension_C|GetSalles%20rencontrés _gi_ascension_3)))
                            (for _array_element_2 _keys
                              (if (== _array_element_2 (Variables|/Game/GI_Ascension.GI_Ascension_C|GetDerniereSalle _gi_ascension_3))
                                (Utilities|Map|Add (Variables|/Game/GI_Ascension.GI_Ascension_C|GetSalles%20rencontrés (Variables|Default|GetGI%20Ascension)) _array_element_2 (+ (.Value (Utilities|Map|Find (Variables|/Game/GI_Ascension.GI_Ascension_C|GetSalles%20rencontrés (Variables|Default|GetGI%20Ascension)) _array_element_2)) 1.0))))
                            (Variables|/Game/GI_Ascension.GI_Ascension_C|SetChoice2 (Variables|Default|GetGI%20Ascension) 0)
                            (CallFunction|PourcentageSallesRencontrés)
                            (CallFunction|DifférenceSouhaitéEtRéel)
                            (CallFunction|EvenementsSalles))))))))))))
      (:then_1
        (Variables|/Game/GI_Ascension.GI_Ascension_C|SetPremier%20Lancement%20MAIN (Variables|Default|GetGI%20Ascension) false)))))

(event Custom|At%20destination
  (if (Utilities|Operators|EqualEqual (Transformation|GetWorldLocation (Variables|Default|GetDestination)) (Transformation|GetWorldLocation (Variables|/Script/Engine.Character|GetMesh (Variables|Default|GetPlayer))) 5e+01)
    (Utilities|FlowControl|DoOnce false
      (:Completed
        (Input|SetInputModeGameandUI (Game|GetPlayerController 0) 0 "DoNotLock" true false)))))

(event EventBeginPlay
  (Utilities|FlowControl|Sequence
    (:then_0
      ;[1 0.4922 0] Références
      (bind _asgi_ascension (Utilities|Casting|CastToGI_Ascension (Game|GetGameInstance)))
      (Variables|Default|SetGI%20Ascension _asgi_ascension)
      (bind _asbp_third_person_character (Utilities|Casting|CastToBP_ThirdPersonCharacter (Game|GetPlayerCharacter 0)))
      (Variables|Default|SetPlayer _asbp_third_person_character))
    (:then_1
      (Utilities|FlowControl|Delay 0.1)
      (CallFunction|EvenementsSalles)
      (Rendering|Components|TextRender|SetText (Variables|Default|Getid_) (Utilities|Text|ToText(Integer) (Variables|Default|GetID))))))

(fn ConstructionScript)

(fn ChoixLePlusEloigné
  ;[0 1 0.1328] Séléction de la salle la plus éloigné du pourcentage souhaité
  (Variables|1erChoix|SetIndex%20le%20plus%20éloigner 0)
  (Variables|1erchoix|SetValeur%20Plus%20Eloigne 0.0)
  (for (_array_element _array_index) (Variables|/Game/GI_Ascension.GI_Ascension_C|GetDifférences%20souhaité/réel (Variables|Default|GetGI%20Ascension))
    (if (> _array_element (Variables|1erchoix|GetValeur%20Plus%20Eloigne))
      (Variables|1erchoix|SetValeur%20Plus%20Eloigne _array_element)
      (Variables|1erChoix|SetIndex%20le%20plus%20éloigner _array_index))))

(fn ChoixDes3PlusÉloignés
  (bind _gi_ascension (Variables|Default|GetGI%20Ascension))
  ;[0.7812 1 0] Copie de la liste de salles dans un array et suppression de l'élément le plus proche de 0
  (bind _output_get (Variables|deuxièmechoix|SetListe2èmeChoix (Variables|/Game/GI_Ascension.GI_Ascension_C|GetListSalles/PourcentageSouhaité _gi_ascension)))
  (bind _keys (Utilities|Map|Keys _output_get))
  (for (_array_element _array_index) _keys
    (if (== _array_index (.IndexOfMaxValue (Math|Float|MaxOfFloatArray (Variables|/Game/GI_Ascension.GI_Ascension_C|GetDifférences%20souhaité/réel _gi_ascension))))
      (Utilities|Map|Remove (Variables|deuxièmechoix|GetListe2èmeChoix) _array_element)
      (Utilities|Array|RemoveIndex (Variables|Default|GetSalles_Icones) _array_index)))
  (bind _keys_2 (Utilities|Map|Keys (Variables|deuxièmechoix|GetListe2èmeChoix)))
  (for (_array_element_2 _array_index_2) _keys_2
    (if (== _array_index_2 (.IndexOfMinValue (Math|Float|MinOfFloatArray (Variables|/Game/GI_Ascension.GI_Ascension_C|GetDifférences%20souhaité/réel (Variables|Default|GetGI%20Ascension)))))
      (Utilities|Map|Remove (Variables|deuxièmechoix|GetListe2èmeChoix) _array_element_2)
      (Utilities|Array|RemoveIndex (Variables|Default|GetSalles_Icones) _array_index_2))))

(fn PourcentageSallesRencontrés
  (bind _gi_ascension (Variables|Default|GetGI%20Ascension))
  ;[1 0 0.2344] Pourcentage des salles rencontrés
  (bind _values (Utilities|Map|Values (Variables|/Game/GI_Ascension.GI_Ascension_C|GetSalles%20rencontrés _gi_ascension)))
  (for (_array_element _array_index) _values
    (Utilities|Array|SetArrayElem (Variables|/Game/GI_Ascension.GI_Ascension_C|GetListSalles/PourcentageRéel _gi_ascension) _array_index (/ _array_element (Variables|/Game/GI_Ascension.GI_Ascension_C|GetSalles%20rencontrés%20total _gi_ascension)))))

(fn DifférenceSouhaitéEtRéel
  (bind _gi_ascension (Variables|Default|GetGI%20Ascension))
  ;[0.9688 0 1] Calcul de la différence entre le pourcentage souhaité et le pourcentage réel
  (bind _values (Utilities|Map|Values (Variables|/Game/GI_Ascension.GI_Ascension_C|GetListSalles/PourcentageSouhaité _gi_ascension)))
  (for (_ _array_index) _values
    (bind _output_get (Variables|Default|SetArray%20Index _array_index))
    (Utilities|Array|SetArrayElem (Variables|/Game/GI_Ascension.GI_Ascension_C|GetDifférences%20souhaité/réel (Variables|Default|GetGI%20Ascension)) _output_get (- (Utilities|Array|Get(acopy) _values (Variables|Default|GetArray%20Index)) (Utilities|Array|Get(acopy) (Variables|/Game/GI_Ascension.GI_Ascension_C|GetListSalles/PourcentageRéel _gi_ascension) (Variables|Default|GetArray%20Index))))))

(fn EvenementsSalles
  (bind _gi_ascension (Variables|Default|GetGI%20Ascension))
  (bind _gi_ascension_2 (Variables|Default|GetGI%20Ascension))
  (bind _gi_ascension_3 (Variables|Default|GetGI%20Ascension))
  (bind _salle_hub (Variables|/Game/GI_Ascension.GI_Ascension_C|GetSalle_Hub _gi_ascension_3))
  (if (== (Variables|/Game/GI_Ascension.GI_Ascension_C|GetSalles%20rencontrés%20total (Variables|Default|GetGI%20Ascension)) 10)
    (bind _returnvalue (UserInterface|CreateWidget "/Game/Widget/Menu/WB_FinduJeu.WB_FinduJeu_C"))
    (UserInterface|Viewport|AddtoViewport _returnvalue 0)
    (else
      (switch int (- (Variables|/Game/GI_Ascension.GI_Ascension_C|GetSalles%20rencontrés%20total _gi_ascension) (Variables|/Game/GI_Ascension.GI_Ascension_C|GetProchaineSalleHUB _gi_ascension))
        (:Default
          ;[1 0.4219 0] Proposition de salle en fonction de l'ascenseur
          (switch int (Variables|Default|GetID) :!label _label
            (:0
              ;[0 1 0.01562] Choisi la salle la plus éloigné de 0
              (CallFunction|ChoixLePlusEloigné)
              (bind _keys (Utilities|Map|Keys (Variables|/Game/GI_Ascension.GI_Ascension_C|GetListSalles/PourcentageSouhaité (Variables|Default|GetGI%20Ascension))))
              (bind _outactors (Actor|GetAllActorsOfClass "BP_Ascenseur_C"))
              (for _array_element _outactors
                (if (== (Variables|BP_Ascenseur_C|GetID _array_element) (Variables|Default|GetID))
                  (bind _output_get (Variables|/Game/GI_Ascension.GI_Ascension_C|SetChoice1 (Variables|Default|GetGI%20Ascension) (Utilities|Array|Get(acopy) _keys (Variables|1erChoix|GetIndex%20le%20plus%20éloigner))))
                  (Rendering|Components|TextRender|SetText (Variables|BP_Ascenseur_C|GetTxt_Choix _array_element) (Utilities|Text|ToText(String) (Utilities|GetClassDisplayName _output_get)))
                  (Rendering|Components|Sprite|SetSprite (Variables|Default|GetLogo) (Utilities|Array|Get(acopy) (Variables|Default|GetSalles_Icones) (Variables|1erChoix|GetIndex%20le%20plus%20éloigner))))))
            (:1
              ;[0.1719 1 0] Choisir un élément au hasard parmis les plus éloignés
              (CallFunction|ChoixDes3PlusÉloignés)
              (bind _outactors_2 (Actor|GetAllActorsOfClass "BP_Ascenseur_C"))
              (for _array_element_2 _outactors_2
                (if (== (Variables|BP_Ascenseur_C|GetID _array_element_2) (Variables|Default|GetID))
                  (if (== (Variables|/Game/GI_Ascension.GI_Ascension_C|GetChoice2 (Variables|Default|GetGI%20Ascension)) 0)
                    (bind _keys_2 (Utilities|Map|Keys (Variables|deuxièmechoix|GetListe2èmeChoix)))
                    (bind _output_get_2 (Variables|Default|SetNewVar_0 (Math|Random|RandomInteger (Utilities|Array|Length _keys_2))))
                    (bind _output_get_3 (Variables|/Game/GI_Ascension.GI_Ascension_C|SetChoice2 (Variables|Default|GetGI%20Ascension) (Utilities|Array|Get(acopy) _keys_2 _output_get_2)))
                    (Rendering|Components|TextRender|SetText (Variables|BP_Ascenseur_C|GetTxt_Choix _array_element_2) (Utilities|Text|ToText(String) (Utilities|GetClassDisplayName _output_get_3)))
                    (Rendering|Components|Sprite|SetSprite (Variables|Default|GetLogo) (Utilities|Array|Get(acopy) (Variables|Default|GetSalles_Icones) (Variables|Default|GetNewVar_0)))
                    (else
                      (Rendering|Components|TextRender|SetText (Variables|BP_Ascenseur_C|GetTxt_Choix _array_element_2) (Utilities|Text|ToText(String) (Utilities|GetClassDisplayName (Variables|/Game/GI_Ascension.GI_Ascension_C|GetChoice2 (Variables|Default|GetGI%20Ascension)))))
                      (bind _keys_3 (Utilities|Map|Keys (Variables|deuxièmechoix|GetListe2èmeChoix)))
                      (for (_array_element_3 _array_index) _keys_3
                        (if (== _array_element_3 (Variables|/Game/GI_Ascension.GI_Ascension_C|GetChoice2 (Variables|Default|GetGI%20Ascension)))
                          (Rendering|Components|Sprite|SetSprite (Variables|Default|GetLogo) (Utilities|Array|Get(acopy) (Variables|Default|GetSalles_Icones) _array_index)))))))))))
        (:-2
          ;[1 0.2578 0] Les salles proposés ne sont que des Combats
          (bind _keys_4 (Utilities|Map|Keys (Variables|/Game/GI_Ascension.GI_Ascension_C|GetListSalles/PourcentageSouhaité _gi_ascension_2)))
          (bind _outactors_3 (Actor|GetAllActorsOfClass "BP_Ascenseur_C"))
          (for _array_element_4 _outactors_3
            (bind _output_get_4 (Variables|/Game/GI_Ascension.GI_Ascension_C|SetChoice1 _gi_ascension_2 (Utilities|Array|Get(acopy) _keys_4)))
            (Variables|/Game/GI_Ascension.GI_Ascension_C|SetChoice2 _gi_ascension_2 _output_get_4)
            (Rendering|Components|TextRender|SetText (Variables|BP_Ascenseur_C|GetTxt_Choix _array_element_4) (Utilities|Text|ToText(String) (Utilities|GetClassDisplayName (Utilities|Array|Get(acopy) _keys_4))))))
        (:-1
          ;[0.9219 1 0] Les salles proposés ne sont que des HUBS
          (bind _outactors_4 (Actor|GetAllActorsOfClass "BP_Ascenseur_C"))
          (for _array_element_5 _outactors_4
            (bind _output_get_5 (Variables|/Game/GI_Ascension.GI_Ascension_C|SetChoice1 _gi_ascension_3 _salle_hub))
            (Variables|/Game/GI_Ascension.GI_Ascension_C|SetChoice2 _gi_ascension_3 _output_get_5)
            (Rendering|Components|TextRender|SetText (Variables|BP_Ascenseur_C|GetTxt_Choix _array_element_5) (Utilities|Text|ToText(String) (Utilities|GetClassDisplayName _salle_hub)))
            (Rendering|Components|Sprite|SetSprite (Variables|Default|GetLogo) "/Game/Environnement/Salles/Icones/HUB_Sprite.HUB_Sprite")))
        (:0
          ;[1 0 0.8906] Mise à jour de la variable "Prochaine salle HUB"
          (Variables|/Game/GI_Ascension.GI_Ascension_C|SetProchaineSalleHUB (Variables|Default|GetGI%20Ascension) (+ (Variables|/Game/GI_Ascension.GI_Ascension_C|GetProchaineSalleHUB (Variables|Default|GetGI%20Ascension)) 10))
          (goto _label))))))