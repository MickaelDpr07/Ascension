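; Combat room Blueprint that sets up camera switching and spawns the room's two elevators.
; On BeginPlay, once the GI_Ascension cast succeeds, it switches the camera to SpawnCamera1 and spawns a BP_Ascenseur at the left and right elevator markers, each with an incrementing ID.
; Any overlap with its Box switches the camera to the SpawnCamera location.
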(event OnComponentBeginOverlap(Box)
  (params (OverlappedComponent :type Primitive%20Component%20Object%20Reference) (OtherActor :type Actor%20Object%20Reference) (OtherComp :type Primitive%20Component%20Object%20Reference) (OtherBodyIndex :type Integer) (bFromSweep :type Boolean) (SweepResult :type Hit%20Result%20Structure%20%28by%20ref%29))
  (CallFunction|CameraSwitch (Transformation|GetWorldLocation (Variables|Default|GetSpawn%20Camera))))

(event EventBeginPlay
  (bind _id_spawn_ascenseur (Variables|Default|GetID_Spawn_Ascenseur))
  (Utilities|Casting|CastToGI_Ascension (Game|GetGameInstance))
  (Utilities|FlowControl|Sequence
    (:then_0
      (CallFunction|CameraSwitch (Transformation|GetWorldLocation (Variables|Default|GetSpawn%20Camera1))))
    (:then_1
      (for _array_element (Utilities|Array|MakeArray (Variables|Default|GetAscenseur%20de%20Gauche) (Variables|Default|GetAscenseur%20de%20Droite))
        (bind _returnvalue (Game|SpawnActorfromClass "/Game/Environnement/ETAGE_2/salles/BP_Ascenseur.BP_Ascenseur_C" (Math|Transform|MakeTransform (Transformation|GetWorldLocation _array_element) (Transformation|GetWorldRotation _array_element) "1.000000,1.000000,1.000000") "Undefined" "MultiplyWithRoot" 0 0))
        (Variables|/Game/Environnement/ETAGE_2/salles/BP_Ascenseur.BP_Ascenseur_C|SetID _returnvalue _id_spawn_ascenseur)
        (Math|Integer|IncrementInt _id_spawn_ascenseur)))))

(fn ConstructionScript)