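; BP_Portail is an environment gate that lowers once when the player interacts with it from inside its trigger box.
; Box overlap shows the Interact prompt and flags the player as in range, as long as IsDone is still true.
; A looping timer polls that flag and the character's Interract variable rather than binding input.
; When both are true, a DoOnce plays a timeline that slides Portail down, hides the prompt and clears IsDone.
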(event OnComponentBeginOverlap(Box)
  (params (OverlappedComponent :type Primitive%20Component%20Object%20Reference) (OtherActor :type Actor%20Object%20Reference) (OtherComp :type Primitive%20Component%20Object%20Reference) (OtherBodyIndex :type Integer) (bFromSweep :type Boolean) (SweepResult :type Hit%20Result%20Structure%20%28by%20ref%29))
  (if (and (== OtherActor (Variables|Default|GetJoueur)) (Variables|Default|GetisDone))
    (Variables|Default|SetInterract? true)
    (Rendering|SetVisibility (Variables|Default|GetInteract) true false)))

(event OnComponentEndOverlap(Box)
  (params (OverlappedComponent :type Primitive%20Component%20Object%20Reference) (OtherActor :type Actor%20Object%20Reference) (OtherComp :type Primitive%20Component%20Object%20Reference) (OtherBodyIndex :type Integer))
  (if (== OtherActor (Variables|Default|GetJoueur))
    (Variables|Default|SetInterract? false)
    (Rendering|SetVisibility (Variables|Default|GetInteract) false false)))

(event Custom|Go_Down
  (if (and (Variables|/Game/ThirdPerson/Blueprints/BP_ThirdPersonCharacter.BP_ThirdPersonCharacter_C|GetInterract (Variables|Default|GetJoueur)) (Variables|Default|GetInterract?))
    (Utilities|FlowControl|DoOnce false
      (:Completed
        (bind _newtrack_0 (Timeline|Timeline PlayFromStart)
          (:Update
            (Transformation|SetRelativeLocation (Variables|Default|GetPortail) (Math|Vector|MakeVector 5e+01 1.5e+02 (Math|Float|Lerp 0.0 -201.0 _newtrack_0)) false false)
            (Rendering|SetVisibility (Variables|Default|GetInteract) false false)
            (Variables|Default|SetisDone false)))))))

(event EventBeginPlay
  (Utilities|Time|SetTimerbyEvent (delegate Custom|Go_Down) 0.05 true)
  (bind _asbp_third_person_character (Utilities|Casting|CastToBP_ThirdPersonCharacter (Game|GetPlayerCharacter 0)))
  (Variables|Default|SetJoueur _asbp_third_person_character))

(fn ConstructionScript)