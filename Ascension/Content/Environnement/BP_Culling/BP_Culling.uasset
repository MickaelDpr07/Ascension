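; BP_Culling is a trigger volume that animates a material blend on a referenced actor as the third-person player enters and leaves.
; It caches the player on BeginPlay and responds only to its capsule overlapping the Box.
; Entry plays one Timeline forward and exit reverses a second, separate one, each driving the actor's BlendDistance material scalar through a scaled track.
; Debug messages print on both overlaps.
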(event OnComponentBeginOverlap(Box)
  (params (OverlappedComponent :type Primitive%20Component%20Object%20Reference) (OtherActor :type Actor%20Object%20Reference) (OtherComp :type Primitive%20Component%20Object%20Reference) (OtherBodyIndex :type Integer) (bFromSweep :type Boolean) (SweepResult :type Hit%20Result%20Structure%20%28by%20ref%29))
  (if (== OtherComp (Variables|/Script/Engine.Character|GetCapsuleComponent (Variables|Default|GetPlayer)))
    (Development|PrintString "Hello")
    (bind _newtrack_0 (Timeline|Timeline PlayFromStart)
      (:Update
        (Rendering|Material|SetScalarParameterValueonMaterials (Variables|Default|GetActor) "BlendDistance" (* _newtrack_0 2e+03))))))

(event OnComponentEndOverlap(Box)
  (params (OverlappedComponent :type Primitive%20Component%20Object%20Reference) (OtherActor :type Actor%20Object%20Reference) (OtherComp :type Primitive%20Component%20Object%20Reference) (OtherBodyIndex :type Integer))
  (if (== OtherComp (Variables|/Script/Engine.Character|GetCapsuleComponent (Variables|Default|GetPlayer)))
    (Development|PrintString "Bye")
    (bind _newtrack_0 (Timeline|Timeline_0 ReverseFromEnd)
      (:Update
        (Rendering|Material|SetScalarParameterValueonMaterials (Variables|Default|GetActor) "BlendDistance" (* _newtrack_0 2e+03))))))

(event EventBeginPlay
  (bind _asbp_third_person_character (Utilities|Casting|CastToBP_ThirdPersonCharacter (Game|GetPlayerCharacter 0)))
  (Variables|Default|SetPlayer _asbp_third_person_character))

(fn ConstructionScript)