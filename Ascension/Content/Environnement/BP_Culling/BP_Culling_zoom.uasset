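; Trigger volume that drives a material blend and adjusts the third-person camera's X distance while the player is inside.
; Overlapping the box with the player capsule plays timelines that scale the "BlendDistance" material parameter on Actor, reversing on exit.
; While inside, Tick sets the camera's DistanceX to an offset behind the player's X position.
; Exiting restores the DistanceX cached at BeginPlay.
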(event OnComponentBeginOverlap(Box)
  (params (OverlappedComponent :type Primitive%20Component%20Object%20Reference) (OtherActor :type Actor%20Object%20Reference) (OtherComp :type Primitive%20Component%20Object%20Reference) (OtherBodyIndex :type Integer) (bFromSweep :type Boolean) (SweepResult :type Hit%20Result%20Structure%20%28by%20ref%29))
  (if (== OtherComp (Variables|/Script/Engine.Character|GetCapsuleComponent (Variables|Default|GetPlayer)))
    (Development|PrintString "Hello")
    (bind _newtrack_0 (Timeline|Timeline PlayFromStart)
      (:Update
        (Rendering|Material|SetScalarParameterValueonMaterials (Variables|Default|GetActor) "BlendDistance" (* _newtrack_0 1e+04))
        (Variables|Default|SetJoueurdansbox true)))))

(event OnComponentEndOverlap(Box)
  (params (OverlappedComponent :type Primitive%20Component%20Object%20Reference) (OtherActor :type Actor%20Object%20Reference) (OtherComp :type Primitive%20Component%20Object%20Reference) (OtherBodyIndex :type Integer))
  (if (== OtherComp (Variables|/Script/Engine.Character|GetCapsuleComponent (Variables|Default|GetPlayer)))
    (Development|PrintString "Bye")
    (bind _newtrack_0 (Timeline|Timeline_0 ReverseFromEnd)
      (:Update
        (Rendering|Material|SetScalarParameterValueonMaterials (Variables|Default|GetActor) "BlendDistance" (* _newtrack_0 1e+04))
        (Variables|Default|SetJoueurdansbox false)
        (Variables|/Game/ThirdPerson/Blueprints/BP_Camera_ThirdPerson.BP_Camera_ThirdPerson_C|SetDistance%20X (Variables|Default|GetCamera) (Variables|Default|GetDistance%20X%20camera))))))

(event EventBeginPlay
  (bind _asbp_third_person_character (Utilities|Casting|CastToBP_ThirdPersonCharacter (Game|GetPlayerCharacter 0)))
  (Variables|Default|SetPlayer _asbp_third_person_character)
  (bind _returnvalue (Actor|GetActorOfClass "/Game/ThirdPerson/Blueprints/BP_Camera_ThirdPerson.BP_Camera_ThirdPerson_C"))
  (Variables|Default|SetCamera _returnvalue)
  (Variables|Default|SetDistance%20X%20camera (Variables|/Game/ThirdPerson/Blueprints/BP_Camera_ThirdPerson.BP_Camera_ThirdPerson_C|GetDistance%20X (Variables|Default|GetCamera))))

(event EventTick
  (params (DeltaSeconds :type Float%20%28single-precision%29))
  (if (Variables|Default|GetJoueurdansbox)
    (Variables|/Game/ThirdPerson/Blueprints/BP_Camera_ThirdPerson.BP_Camera_ThirdPerson_C|SetDistance%20X (Variables|Default|GetCamera) (Math|Float|Lerp (Variables|Default|GetDistance%20X%20camera) (- (.x (Transformation|GetActorLocation (Variables|Default|GetPlayer))) 5e+02) 1.0))))

(fn ConstructionScript)