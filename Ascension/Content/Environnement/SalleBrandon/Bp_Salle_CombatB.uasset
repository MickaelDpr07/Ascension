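; Combat room Blueprint (Salle CombatB) that moves the game camera between two marker positions in the level.
; On BeginPlay, once the GI_Ascension game instance cast succeeds, it calls CameraSwitch with SpawnCamera1's location.
; Any overlap with its Box trigger calls CameraSwitch with SpawnCamera's location, without filtering the overlapping actor.
; BeginPlay also loops over the left and right elevators, but the loop body is empty.
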(event OnComponentBeginOverlap(Box)
  (params (OverlappedComponent :type Primitive%20Component%20Object%20Reference) (OtherActor :type Actor%20Object%20Reference) (OtherComp :type Primitive%20Component%20Object%20Reference) (OtherBodyIndex :type Integer) (bFromSweep :type Boolean) (SweepResult :type Hit%20Result%20Structure%20%28by%20ref%29))
  (CallFunction|CameraSwitch (Transformation|GetWorldLocation (Variables|Default|GetSpawn%20Camera))))

(event EventBeginPlay
  (Utilities|Casting|CastToGI_Ascension (Game|GetGameInstance))
  (Utilities|FlowControl|Sequence
    (:then_0
      (CallFunction|CameraSwitch (Transformation|GetWorldLocation (Variables|Default|GetSpawn%20Camera1))))
    (:then_1
      (for _array_element (Utilities|Array|MakeArray (Variables|Default|GetAscenseur%20de%20Gauche) (Variables|Default|GetAscenseur%20de%20Droite))
        _))))

(fn ConstructionScript)