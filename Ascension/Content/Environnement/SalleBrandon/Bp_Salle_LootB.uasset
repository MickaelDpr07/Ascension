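; Loot room Blueprint (variant B) that sets up the camera and two exit elevators when play begins.
; It caches the GI_Ascension game instance, then calls CameraSwitch with the SpawnCamera component's location.
; After a short delay, it spawns a BP_Ascenseur at the left and right marker transforms, giving each an incrementing ID.
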(event EventBeginPlay
  (bind _id_spawn_ascenseur (Variables|Default|GetID_Spawn_Ascenseur))
  (bind _asgi_ascension (Utilities|Casting|CastToGI_Ascension (Game|GetGameInstance)))
  (Variables|Default|SetGI%20Ascension _asgi_ascension)
  (Utilities|FlowControl|Sequence
    (:then_0
      (CallFunction|CameraSwitch (Transformation|GetWorldLocation (Variables|Default|GetSpawn%20Camera))))
    (:then_1
      (Utilities|FlowControl|Delay 2.0)
      (for _array_element (Utilities|Array|MakeArray (Variables|Default|GetAscenseur%20de%20Gauche) (Variables|Default|GetAscenseur%20de%20Droite))
        (bind _returnvalue (Game|SpawnActorfromClass "/Game/Environnement/ETAGE_2/salles/Ascenseur/BP_Ascenseur.BP_Ascenseur_C" (Math|Transform|MakeTransform (Transformation|GetWorldLocation _array_element) (Transformation|GetWorldRotation _array_element) "1.000000,1.000000,1.000000") "Undefined" "MultiplyWithRoot" 0 0))
        (Variables|/Game/Environnement/ETAGE_2/salles/Ascenseur/BP_Ascenseur.BP_Ascenseur_C|SetID _returnvalue _id_spawn_ascenseur)
        (Math|Integer|IncrementInt _id_spawn_ascenseur)))))

(fn ConstructionScript)