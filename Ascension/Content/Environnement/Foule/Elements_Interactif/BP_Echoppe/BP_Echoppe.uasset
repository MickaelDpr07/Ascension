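; BP_Echoppe is an interactive market stall in the crowd environment that detects crowd characters (BP_Foule) near it.
; Entering or leaving the Detection component toggles the character's CharacterInEchoppe flag and the IsChecking Blackboard key that feeds its AI.
; The construction script gathers three queue references (BPFileAttente) into the FileDattente array, which this file's graphs do not otherwise use.
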(event OnComponentBeginOverlap(Detection)
  (params (OverlappedComponent :type Primitive%20Component%20Object%20Reference) (OtherActor :type Actor%20Object%20Reference) (OtherComp :type Primitive%20Component%20Object%20Reference) (OtherBodyIndex :type Integer) (bFromSweep :type Boolean) (SweepResult :type Hit%20Result%20Structure%20%28by%20ref%29))
  (bind _asbp_foule (Utilities|Casting|CastToBP_Foule OtherActor))
  (bind _output_get (Variables|Default|SetAs%20BP%20Foule _asbp_foule))
  (Variables|/Game/Environnement/Foule/BP_Foule.BP_Foule_C|SetCharacterInEchoppe _output_get true)
  (AI|Components|Blackboard|SetValueasBool (AI|GetBlackboard _output_get) (Utilities|Name|MakeLiteralName "IsChecking") true))

(event OnComponentEndOverlap(Detection)
  (params (OverlappedComponent :type Primitive%20Component%20Object%20Reference) (OtherActor :type Actor%20Object%20Reference) (OtherComp :type Primitive%20Component%20Object%20Reference) (OtherBodyIndex :type Integer))
  (bind _asbp_foule (Utilities|Casting|CastToBP_Foule OtherActor))
  (bind _output_get (Variables|Default|SetAs%20BP%20Foule _asbp_foule))
  (Variables|/Game/Environnement/Foule/BP_Foule.BP_Foule_C|SetCharacterInEchoppe _output_get false)
  (AI|Components|Blackboard|SetValueasBool (AI|GetBlackboard _output_get) (Utilities|Name|MakeLiteralName "IsChecking") false))

(event EventBeginPlay)

(fn ConstructionScript
  (Variables|Default|SetFileD'attente (Utilities|Array|MakeArray (Variables|Default|GetBP_FileAttente) (Variables|Default|GetBP_FileAttente1) (Variables|Default|GetBP_FileAttente2))))