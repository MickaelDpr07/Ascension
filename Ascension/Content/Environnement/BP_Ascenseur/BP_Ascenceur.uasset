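; Elevator actor that switches the camera while the player is inside and opens the elevator's level widget.
; Box overlaps blend the view between the Camera child actor and the third-person camera, using two DoOnce gates that re-arm each other.
; When the player overlaps Detection, it creates the WB_Ascenseur widget and passes it the current, upper and lower levels.
; BeginPlay caches the player, default camera and GI_Ascension game instance.
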(event OnComponentBeginOverlap(Box)
  (params (OverlappedComponent :type Primitive%20Component%20Object%20Reference) (OtherActor :type Actor%20Object%20Reference) (OtherComp :type Primitive%20Component%20Object%20Reference) (OtherBodyIndex :type Integer) (bFromSweep :type Boolean) (SweepResult :type Hit%20Result%20Structure%20%28by%20ref%29))
  (if (== OtherComp (Variables|/Script/Engine.Character|GetCapsuleComponent (Variables|Default|GetPlayer)))
    (Variables|Default|SetCharacterInBox true)
    (CallFunction|CameraMovment)))

(event OnComponentEndOverlap(Box)
  (params (OverlappedComponent :type Primitive%20Component%20Object%20Reference) (OtherActor :type Actor%20Object%20Reference) (OtherComp :type Primitive%20Component%20Object%20Reference) (OtherBodyIndex :type Integer))
  (if (== OtherComp (Variables|/Script/Engine.Character|GetCapsuleComponent (Variables|Default|GetPlayer)))
    (Variables|Default|SetCharacterInBox false)
    (CallFunction|CameraReset)))

(event OnComponentBeginOverlap(Detection)
  (params (OverlappedComponent :type Primitive%20Component%20Object%20Reference) (OtherActor :type Actor%20Object%20Reference) (OtherComp :type Primitive%20Component%20Object%20Reference) (OtherBodyIndex :type Integer) (bFromSweep :type Boolean) (SweepResult :type Hit%20Result%20Structure%20%28by%20ref%29))
  ;[0.07812 0 1] Affichage widget quand le joueur entre en collision avec le boutton de l'ascenseur
  (if (== OtherActor (Variables|Default|GetPlayer))
    (CallFunction|OuvertureWidget+AssigniationLevel)))

(event Custom|Ouverture%20Widget%20+%20assigniation%20level
  (bind _returnvalue (UserInterface|CreateWidget "/Game/Widget/Ascenseur/WB_Ascenseur.WB_Ascenseur_C" (Game|GetPlayerController 0)))
  (UserInterface|Viewport|AddtoViewport _returnvalue 0)
  (Variables|/Game/Widget/Ascenseur/WB_Ascenseur.WB_Ascenseur_C|SetLevel%20Actuel _returnvalue (Variables|Default|GetLevel%20Actuel))
  (Variables|/Game/Widget/Ascenseur/WB_Ascenseur.WB_Ascenseur_C|SetLevel%20Suivant%20à%20Charger _returnvalue (Variables|Default|GetLevel%20Supérieur))
  (Variables|/Game/Widget/Ascenseur/WB_Ascenseur.WB_Ascenseur_C|SetLevel%20Inférieur _returnvalue (Variables|Default|GetLevel%20Inférieur)))

(event Custom|CameraMovment
  ;[0.4397 0.9911 1] Set Caméra
  (if (Variables|Default|GetCharacterInBox)
    (Utilities|FlowControl|DoOnce false
      (:Completed
        (Game|Player|SetViewTargetwithBlend (Game|GetPlayerController 0) (Variables|/Script/Engine.ChildActorComponent|GetChildActor (Variables|Default|GetCamera)) 0.0 "VTBlend_Linear" 0.0 false)
        (CallFunction|ResetCam)))))

(event Custom|Set%20Cam
  ;[0.4397 0.9911 1] Set Caméra
  (Utilities|FlowControl|DoOnce false) ; enters at Reset
)

(event Custom|CameraReset
  ;[0.4397 0.9911 1] Reset caméra
  (if (not (Variables|Default|GetCharacterInBox))
    (Utilities|FlowControl|DoOnce false
      (:Completed
        (Game|Player|SetViewTargetwithBlend (Game|GetPlayerController 0) (Variables|Default|GetCam) 0.0 "VTBlend_Linear" 0.0 false)
        (CallFunction|SetCam)))))

(event Custom|ResetCam
  ;[0.4397 0.9911 1] Reset caméra
  (Utilities|FlowControl|DoOnce false) ; enters at Reset
)

(event EventBeginPlay
  (Utilities|FlowControl|Sequence
    (:then_0
      (bind _asbp_third_person_character (Utilities|Casting|CastToBP_ThirdPersonCharacter (Game|GetPlayerCharacter 0)))
      (Variables|Default|SetPlayer _asbp_third_person_character)
      (bind _returnvalue (Actor|GetActorOfClass "/Game/ThirdPerson/Blueprints/BP_Camera_ThirdPerson.BP_Camera_ThirdPerson_C"))
      (Variables|Default|SetCam _returnvalue))
    (:then_1
      ;[1 0.2344 0] Référence GI_Ascencion
      (bind _asgi_ascension (Utilities|Casting|CastToGI_Ascension (Game|GetGameInstance)))
      (Variables|Default|SetGI%20Ascension _asgi_ascension))))

(fn ConstructionScript)