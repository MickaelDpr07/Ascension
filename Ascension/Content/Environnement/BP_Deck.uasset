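; BP_Deck is an environment Blueprint that shows the WB_ouverture_Deck widget while the player is inside its Collision volume.
; BeginPlay caches player 0's character as a BP_ThirdPersonCharacter, and both overlap events react only to that actor.
; Begin overlap creates a new widget and adds it to the viewport, and end overlap removes it.
; CustomEvent and the construction script are empty.
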(event OnComponentBeginOverlap(Collision)
  (params (OverlappedComponent :type Primitive%20Component%20Object%20Reference) (OtherActor :type Actor%20Object%20Reference) (OtherComp :type Primitive%20Component%20Object%20Reference) (OtherBodyIndex :type Integer) (bFromSweep :type Boolean) (SweepResult :type Hit%20Result%20Structure%20%28by%20ref%29))
  (if (== OtherActor (Variables|Default|GetPlayer))
    (bind _returnvalue (UserInterface|CreateWidget "/Game/Widget/Deck/WB_ouverture_Deck.WB_ouverture_Deck_C"))
    (bind _output_get (Variables|Default|SetWidget _returnvalue))
    (UserInterface|Viewport|AddtoViewport _output_get 0)))

(event OnComponentEndOverlap(Collision)
  (params (OverlappedComponent :type Primitive%20Component%20Object%20Reference) (OtherActor :type Actor%20Object%20Reference) (OtherComp :type Primitive%20Component%20Object%20Reference) (OtherBodyIndex :type Integer))
  (if (== OtherActor (Variables|Default|GetPlayer))
    (Widget|RemovefromParent (Variables|Default|GetWidget))))

(event Custom|CustomEvent
  (params (OverlappedComponent :type Primitive%20Component%20Object%20Reference) (OtherActor :type Actor%20Object%20Reference) (OtherComp :type Primitive%20Component%20Object%20Reference) (OtherBodyIndex :type Integer)))

(event EventBeginPlay
  (bind _asbp_third_person_character (Utilities|Casting|CastToBP_ThirdPersonCharacter (Game|GetPlayerCharacter 0)))
  (Variables|Default|SetPlayer _asbp_third_person_character))

(fn ConstructionScript)