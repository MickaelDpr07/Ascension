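; Enemy actor for combat that loads the current enemy's stats from data tables and spins for UI display.
; BeginPlay sets hack points, experience, name and fight timer, pushing the latter two to GM_Combat or its widget.
; Up to two defensive effects become flags or regeneration and appear in the widget.
; While unpaused, a one-second Tick countdown drives burn and regeneration through GM_Combat, running only when burn is nonzero.
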(event EventBeginPlay
  (Utilities|FlowControl|Sequence
    (:then_0
      (bind _asgi_ascension (Utilities|Casting|CastToGI_Ascension (Game|GetGameInstance)))
      (Variables|Default|SetGI%20Ascension _asgi_ascension)
      (bind _asgm_combat (Utilities|Casting|CastToGM_Combat (Game|GetGameMode)))
      (Variables|Default|SetGM%20Combat _asgm_combat))
    (:then_1
      (bind _returnvalue (Utilities|GetDataTableRow "/Game/Combat/Systeme/DD_Ennemis.DD_Ennemis" (Utilities|String|StringToName (Utilities|String|ToString(Integer) (Variables|/Game/GI_Ascension.GI_Ascension_C|GetIndex%20Ennemi%20Actuel (Variables|Default|GetGI%20Ascension)))))
        (:then
          (Variables|Default|SetHack%20Max (.Points (Utilities|Struct|BreakSTRUCT_Ennemis _returnvalue)))
          (bind _returnvalue_2 (Utilities|GetDataTableRow "/Game/Combat/Systeme/DD_TypeEnnemis.DD_TypeEnnemis" (Utilities|String|StringToName (Utilities|String|ToString(Integer) (.Type (Utilities|Struct|BreakSTRUCT_Ennemis _returnvalue)))))
            (:then
              (Variables|Default|SetExperience (.Exp (Utilities|Struct|BreakSTRUCT_TypeEnnemis _returnvalue_2)))
              (bind _output_get (Variables|Default|SetNom (.Nom (Utilities|Struct|BreakSTRUCT_Ennemis _returnvalue))))
              (Rendering|Components|TextRender|SetText (Variables|/Game/Widget/Combat/WB_Combat.WB_Combat_C|GetNomEnnemi (Variables|/Game/GM_Combat.GM_Combat_C|GetWB_Combat (Variables|Default|GetGM%20Combat))) _output_get)
              (Variables|/Game/GM_Combat.GM_Combat_C|SetTemps_Total_MAX_Combat (Variables|Default|GetGM%20Combat) (.Temps (Utilities|Struct|BreakSTRUCT_Ennemis _returnvalue)))
              (Variables|/Game/GM_Combat.GM_Combat_C|SetTemps%20Restant%20Combat (Variables|Default|GetGM%20Combat) (.Temps (Utilities|Struct|BreakSTRUCT_Ennemis _returnvalue)))
              ;[1 0.2344 0] Application de (L'/ les) effet(s) défensif sur l'ennemi
              (Utilities|FlowControl|Sequence
                (:then_0
                  ;;[1 0 0.4453] Si l'ennemi à 1 effet defensif : Lui attitre
                  (if (!= (.Effet_Defensif_1 (Utilities|Struct|BreakSTRUCT_Ennemis _returnvalue)) -1)
                    (CallFunction|ApplicationDeL'effetDéfensif (.Effet_Defensif_1 (Utilities|Struct|BreakSTRUCT_Ennemis _returnvalue)))
                    (bind _returnvalue_3 (Utilities|GetDataTableRow "/Game/Combat/Systeme/DD_EffetsDefensif.DD_EffetsDefensif" (Utilities|String|StringToName (Utilities|String|ToString(Integer) (.Effet_Defensif_1 (Utilities|Struct|BreakSTRUCT_Ennemis _returnvalue)))))
                      (:then
                        (Default|AjoutEffetDéfensif (Variables|/Game/GM_Combat.GM_Combat_C|GetWB_Combat (Variables|Default|GetGM%20Combat)) 1 _returnvalue_3)))))
                (:then_1
                  ;;[0.9688 0 1] Si l'ennemi à 2 effets
                  (if (!= (.Effet_Defensif_2 (Utilities|Struct|BreakSTRUCT_Ennemis _returnvalue)) -1)
                    (CallFunction|ApplicationDeL'effetDéfensif (.Effet_Defensif_2 (Utilities|Struct|BreakSTRUCT_Ennemis _returnvalue)))
                    (bind _returnvalue_4 (Utilities|GetDataTableRow "/Game/Combat/Systeme/DD_EffetsDefensif.DD_EffetsDefensif" (Utilities|String|StringToName (Utilities|String|ToString(Integer) (.Effet_Defensif_2 (Utilities|Struct|BreakSTRUCT_Ennemis _returnvalue)))))
                      (:then
                        (Default|AjoutEffetDéfensif (Variables|/Game/GM_Combat.GM_Combat_C|GetWB_Combat (Variables|Default|GetGM%20Combat)) 2 _returnvalue_4)))))))))))
    (:then_2
      (Variables|Default|SetCompteurTick 1.0))
    (:then_3
      ;[0.3828 0 1] Fait tourner l'ennemi dans l'UI
      (bind _rotation (Timeline|Rotation Play)
        (:Update
          (Transformation|SetActorRotation self (Math|Rotator|MakeRotator 0.0 0.0 (* _rotation 3.6e+02))))))))

(event EventTick
  (params (DeltaSeconds :type Float%20%28single-precision%29))
  ;[1 0 0] EVENT TICKS
  (CallFunction|FCompteurTick DeltaSeconds))

(fn ConstructionScript)

(fn FCompteurTick
  (params (Delta%20Time :type Float%20%28double-precision%29))
  (bind _defensif_régénération (Variables|EffetsDéfensif|GetDEFENSIF_Régénération))
  (if (not (Variables|/Game/GI_Ascension.GI_Ascension_C|GetPause%20du%20Combat%20? (Variables|Default|GetGI%20Ascension)))
    ;[1 0.5391 0] Anti Tick Perpetuel
    (if (!= (Variables|Effets|GetBrulure) 0)
      ;[0.2346 0.4072 0.08022] Compteur de ticks
      (bind _output_get (Variables|Default|SetCompteurTick (- (Variables|Default|GetCompteurTick) Delta%20Time)))
      (if (<= _output_get 0.0)
        (Utilities|FlowControl|Sequence
          (:then_0
            ;[1 0.2917 0.2917] Test Effet Brulûre
            (if (>= (Variables|Effets|GetBrulure) 0)
              (bind _result (Math|Integer|DecrementInt (Variables|Effets|GetBrulure))
                (:%20%20
                  (Default|EffetBrulure (Variables|Default|GetGM%20Combat) (select (== _result -1) 0 (Variables|Effets|GetBrulure)))))))
          (:then_1
            ;[0 1 0.8359] DEFENSIF _ Régénération
            (if (!= _defensif_régénération 0)
              (Default|CoûtAjoutHack (Variables|Default|GetGM%20Combat) (* _defensif_régénération -1))))
          (:then_2
            ;[0.5783 1 0.1979] Réinitialise le Compteur
            (Variables|Default|SetCompteurTick 1.0)))))))

(fn ApplicationDeL'effetDéfensif
  (params (Index%20Effet%20Défensif :type Integer))
  (switch int Index%20Effet%20Défensif
    (:0
      (Variables|EffetsDéfensif|SetDEFENSIF_RésitanceFeu%20? true))
    (:1
      (Variables|EffetsDéfensif|SetDEFENSIF_Régénération 5))
    (:2
      (Variables|EffetsDéfensif|SetDEFENSIF_Bouclier%20? true))
    (:3
      (Variables|EffetsDéfensif|SetDEFENSIF_Anti_Modificateur_Temps%20? true))))