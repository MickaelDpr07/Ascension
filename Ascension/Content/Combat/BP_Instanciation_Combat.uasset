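; Combat trigger actor that picks the room's enemy, shows its name, and launches the combat level when the player overlaps its sphere.
; BeginPlay respawns the last enemy after a lost fight, otherwise randomly draws a regular or boss from DD_Ennemis by zone and room count.
; Draws exclude the three most recently encountered enemies, tracked in the GameInstance.
; Overlap stores the enemy index, shows a launch widget, and briefly disables input before loading.
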(event OnComponentBeginOverlap(Sphere)
  (params (OverlappedComponent :type Primitive%20Component%20Object%20Reference) (OtherActor :type Actor%20Object%20Reference) (OtherComp :type Primitive%20Component%20Object%20Reference) (OtherBodyIndex :type Integer) (bFromSweep :type Boolean) (SweepResult :type Hit%20Result%20Structure%20%28by%20ref%29))
  (bind _returnvalue (Game|GetPlayerController 0))
  (bind _third_person_character (Variables|Default|GetThird%20Person%20Character))
  ;[1 0 0.1172] Lors Overlap Instanciation Combat, lancement Combat ou Tuto Combat
  (if (== OtherActor (Variables|Default|GetThird%20Person%20Character))
    (Variables|/Game/GI_Ascension.GI_Ascension_C|SetIndex%20Ennemi%20Actuel (Variables|Default|GetGI%20Ascension) (Math|Conversions|ToInteger(Byte) (Utilities|String|ToString(Name) (Variables|Default|GetEnnemiGénéré))))
    (bind _returnvalue_2 (UserInterface|CreateWidget "/Game/Widget/HUD_LancemementCombat.HUD_LancemementCombat_C"))
    (UserInterface|Viewport|AddtoViewport _returnvalue_2 0)
    (Input|DisableInput _third_person_character _returnvalue)
    (Utilities|FlowControl|Delay 2.75)
    (Input|EnableInput _third_person_character _returnvalue)
    (Game|OpenLevel(byObjectReference) "/Game/ThirdPerson/Maps/LEVEL_Combat.LEVEL_Combat")))

(event EventBeginPlay
  (Utilities|FlowControl|Sequence
    (:then_0
      ;[0 1 1] Références
      (bind _asgi_ascension (Utilities|Casting|CastToGI_Ascension (Game|GetGameInstance)))
      (Variables|Default|SetGI%20Ascension _asgi_ascension)
      (bind _asbp_third_person_character (Utilities|Casting|CastToBP_ThirdPersonCharacter (Game|GetPlayerCharacter 0)))
      (Variables|Default|SetThird%20Person%20Character _asbp_third_person_character))
    (:then_1
      ;[0 1 1] Si combat perdu alors réaparition du même ennemi précédement affronter
      (if (and (not (Variables|/Game/GI_Ascension.GI_Ascension_C|GetDernier%20Combat%20Gagner%20? (Variables|Default|GetGI%20Ascension))) (!= (Variables|/Game/GI_Ascension.GI_Ascension_C|GetIndex%20Ennemi%20Actuel (Variables|Default|GetGI%20Ascension)) 0))
        (Variables|Default|SetIndex%20Ennemi%20Instancié (Variables|/Game/GI_Ascension.GI_Ascension_C|GetIndex%20Ennemi%20Actuel (Variables|Default|GetGI%20Ascension)))
        (bind _output_get (Variables|Default|SetEnnemiGénéré (Utilities|String|StringToName (Utilities|String|ToString(Integer) (Variables|/Game/GI_Ascension.GI_Ascension_C|GetIndex%20Ennemi%20Actuel (Variables|Default|GetGI%20Ascension))))))
        (bind _returnvalue (Utilities|GetDataTableRow "/Game/Combat/Systeme/DD_Ennemis.DD_Ennemis" _output_get)
          (:then
            (Rendering|Components|TextRender|SetText (Variables|Default|GetIndexEnnemiActu) (.Nom (Utilities|Struct|BreakSTRUCT_Ennemis _returnvalue)))
            (Variables|Default|SetEnnemiSet true)))))
    (:then_2
      (if (not (Variables|Default|GetEnnemiSet))
        ;[0.1719 0 1 1 50] Système procédurale pour déterminer l'ennemis de la salle
        ;;[1 0.498 0] Zone 1 ?
        (if (<= (Variables|/Game/GI_Ascension.GI_Ascension_C|GetSalles%20rencontrés%20total (Variables|Default|GetGI%20Ascension)) 10)
          ;;;[0 1 0.9297] Boss
          (if (== (Variables|/Game/GI_Ascension.GI_Ascension_C|GetSalles%20rencontrés%20total (Variables|Default|GetGI%20Ascension)) 9)
            ;;[1 0 0.1875] Set boss de la première zone
            ;;;[0.3359 1 0] Récupère les boss de la première zone
            (CallFunction|GetEnnemisType 2)
            ;;;[1 0.6126 0.3542] En choisit un au hasard
            (Variables|Default|SetEnnemiGénéré (.OutItem (Utilities|Array|Random (Variables|FonctionEnnemisType|GetArrayEnnemis))))
            ;;;[0.3906 0.8263 1] Set le nom de l'ennemis au dessus de celui ci
            (bind _returnvalue_2 (Utilities|GetDataTableRow "/Game/Combat/Systeme/DD_Ennemis.DD_Ennemis" (Variables|Default|GetEnnemiGénéré))
              (:then
                (Rendering|Components|TextRender|SetText (Variables|Default|GetIndexEnnemiActu) (.Nom (Utilities|Struct|BreakSTRUCT_Ennemis _returnvalue_2)))
                ;;;[1 0.3565 0] Permet de savoir les 3 derniers ennemis rencontrés
                (CallFunction|SetArrayEnnemisRencontré)))
            (else
              ;;[1 0 0.1875] Set ennemi de base de la première zone
              ;;;[0.3359 1 0] Récupère les ennemis de base de la première zone
              (CallFunction|GetEnnemisType 1)
              ;;;[1 0.6126 0.3542] En choisit un au hasard
              (Variables|Default|SetEnnemiGénéré (.OutItem (Utilities|Array|Random (Variables|FonctionEnnemisType|GetArrayEnnemis))))
              ;;;[0.3906 0.8263 1] Set le nom de l'ennemis au dessus de celui ci
              (bind _returnvalue_3 (Utilities|GetDataTableRow "/Game/Combat/Systeme/DD_Ennemis.DD_Ennemis" (Variables|Default|GetEnnemiGénéré))
                (:then
                  (Rendering|Components|TextRender|SetText (Variables|Default|GetIndexEnnemiActu) (.Nom (Utilities|Struct|BreakSTRUCT_Ennemis _returnvalue_3)))
                  ;;;[1 0.3565 0] Permet de savoir les 3 derniers ennemis rencontrés
                  (CallFunction|SetArrayEnnemisRencontré)))))
          (else
            ;;[1 0.498 0] Zone 2 ?
            (if (<= (Variables|/Game/GI_Ascension.GI_Ascension_C|GetSalles%20rencontrés%20total (Variables|Default|GetGI%20Ascension)) 20)
              ;;;[0 1 0.9297] Boss
              (if (== (Variables|/Game/GI_Ascension.GI_Ascension_C|GetSalles%20rencontrés%20total (Variables|Default|GetGI%20Ascension)) 19)
                ;;[1 0 0.1875] Set boss de la deuxième zone
                ;;;[0.3359 1 0] Récupère les boss de la deuxième zone
                (CallFunction|GetEnnemisType 4)
                ;;;[1 0.6126 0.3542] En choisit un au hasard
                (Variables|Default|SetEnnemiGénéré (.OutItem (Utilities|Array|Random (Variables|FonctionEnnemisType|GetArrayEnnemis))))
                ;;;[0.3906 0.8263 1] Set le nom de l'ennemis au dessus de celui ci
                (bind _returnvalue_4 (Utilities|GetDataTableRow "/Game/Combat/Systeme/DD_Ennemis.DD_Ennemis" (Variables|Default|GetEnnemiGénéré))
                  (:then
                    (Rendering|Components|TextRender|SetText (Variables|Default|GetIndexEnnemiActu) (.Nom (Utilities|Struct|BreakSTRUCT_Ennemis _returnvalue_4)))
                    ;;;[1 0.3565 0] Permet de savoir les 3 derniers ennemis rencontrés
                    (CallFunction|SetArrayEnnemisRencontré)))
                (else
                  ;;[1 0 0.1875] Set ennemi de base de la deuxième zone
                  ;;;[0.3359 1 0] Récupère les ennemis de base de la deuxième zone
                  (CallFunction|GetEnnemisType 3)
                  ;;;[1 0.6126 0.3542] En choisit un au hasard
                  (Variables|Default|SetEnnemiGénéré (.OutItem (Utilities|Array|Random (Variables|FonctionEnnemisType|GetArrayEnnemis))))
                  ;;;[0.3906 0.8263 1] Set le nom de l'ennemis au dessus de celui ci
                  (bind _returnvalue_5 (Utilities|GetDataTableRow "/Game/Combat/Systeme/DD_Ennemis.DD_Ennemis" (Variables|Default|GetEnnemiGénéré))
                    (:then
                      (Rendering|Components|TextRender|SetText (Variables|Default|GetIndexEnnemiActu) (.Nom (Utilities|Struct|BreakSTRUCT_Ennemis _returnvalue_5)))
                      ;;;[1 0.3565 0] Permet de savoir les 3 derniers ennemis rencontrés
                      (CallFunction|SetArrayEnnemisRencontré)))))
              (else
                ;;[1 0.498 0] Zone 2 ?
                (if (<= (Variables|/Game/GI_Ascension.GI_Ascension_C|GetSalles%20rencontrés%20total (Variables|Default|GetGI%20Ascension)) 30)
                  ;;;[0 1 0.9297] Boss ?
                  (if (== (Variables|/Game/GI_Ascension.GI_Ascension_C|GetSalles%20rencontrés%20total (Variables|Default|GetGI%20Ascension)) 29)
                    ;;[1 0 0.1875] Set boss de la troisième zone
                    ;;;[0.3359 1 0] Récupère les boss de la troisième zone
                    (CallFunction|GetEnnemisType 6)
                    ;;;[1 0.6126 0.3542] En choisit un au hasard
                    (Variables|Default|SetEnnemiGénéré (.OutItem (Utilities|Array|Random (Variables|FonctionEnnemisType|GetArrayEnnemis))))
                    ;;;[0.3906 0.8263 1] Set le nom de l'ennemis au dessus de celui ci
                    (bind _returnvalue_6 (Utilities|GetDataTableRow "/Game/Combat/Systeme/DD_Ennemis.DD_Ennemis" (Variables|Default|GetEnnemiGénéré))
                      (:then
                        (Rendering|Components|TextRender|SetText (Variables|Default|GetIndexEnnemiActu) (.Nom (Utilities|Struct|BreakSTRUCT_Ennemis _returnvalue_6)))
                        ;;;[1 0.3565 0] Permet de savoir les 3 derniers ennemis rencontrés
                        (CallFunction|SetArrayEnnemisRencontré)))
                    (else
                      ;;[1 0 0.1875] Set ennemi de base de la troisième zone
                      ;;;[0.3359 1 0] Récupère les ennemis de base de la troisième zone
                      (CallFunction|GetEnnemisType 5)
                      ;;;[1 0.6126 0.3542] En choisit un au hasard
                      (Variables|Default|SetEnnemiGénéré (.OutItem (Utilities|Array|Random (Variables|FonctionEnnemisType|GetArrayEnnemis))))
                      ;;;[0.3906 0.8263 1] Set le nom de l'ennemis au dessus de celui ci
                      (bind _returnvalue_7 (Utilities|GetDataTableRow "/Game/Combat/Systeme/DD_Ennemis.DD_Ennemis" (Variables|Default|GetEnnemiGénéré))
                        (:then
                          (Rendering|Components|TextRender|SetText (Variables|Default|GetIndexEnnemiActu) (.Nom (Utilities|Struct|BreakSTRUCT_Ennemis _returnvalue_7)))
                          ;;;[1 0.3565 0] Permet de savoir les 3 derniers ennemis rencontrés
                          (CallFunction|SetArrayEnnemisRencontré))))))))))))))

(fn ConstructionScript
  ;[0.9688 1 0] Ajoute le nom de l'ennemi au dessus de sa tête lorsque son ID lui est attribué
  (if (Variables|Default|GetEnnemiSet)
    (bind _output_get (Variables|Default|SetEnnemiGénéré (Utilities|String|StringToName (Utilities|String|ToString(Integer) (Variables|Default|GetIndex%20Ennemi%20Instancié)))))
    (bind _returnvalue (Utilities|GetDataTableRow "/Game/Combat/Systeme/DD_Ennemis.DD_Ennemis" _output_get)
      (:then
        (Rendering|Components|TextRender|SetText (Variables|Default|GetIndexEnnemiActu) (.Nom (Utilities|Struct|BreakSTRUCT_Ennemis _returnvalue)))))))

(fn GetEnnemisType
  (params (Type :type Integer))
  ;[0.3125 1 0] Set le type et récupère la data table des ennemis
  (Variables|FonctionEnnemisType|SetTypeFunction Type)
  (bind _outrownames (DataTable|GetDataTableRowNames (Variables|Default|GetDD_Ennemi)))
  ;[0.7578 1 0] For each loop pour récupérer tous les ennemis du type donné et en faire un array
  (for _array_element _outrownames
    (bind _returnvalue (Utilities|GetDataTableRow "/Game/Combat/Systeme/DD_Ennemis.DD_Ennemis" _array_element)
      (:then
        (if (== (.Type (Utilities|Struct|BreakSTRUCT_Ennemis _returnvalue)) (Variables|FonctionEnnemisType|GetTypeFunction))
          (Utilities|Array|Add (Variables|FonctionEnnemisType|GetArrayEnnemis) _array_element)))))
  ;[0.2422 1 0] Retire les ennemis rencontrés récemment de l'array
  (for _array_element_2 (Variables|/Game/GI_Ascension.GI_Ascension_C|GetEnnemis%20Rencontré%20Récemment (Variables|Default|GetGI%20Ascension))
    (Utilities|Array|RemoveItem (Variables|FonctionEnnemisType|GetArrayEnnemis) _array_element_2)))

(fn SetArrayEnnemisRencontré
  (bind _gi_ascension (Variables|Default|GetGI%20Ascension))
  (bind _gi_ascension_2 (Variables|Default|GetGI%20Ascension))
  (bind _ennemis_rencontré_récemment (Variables|/Game/GI_Ascension.GI_Ascension_C|GetEnnemis%20Rencontré%20Récemment _gi_ascension))
  (bind _ennemis_rencontré_récemment_2 (Variables|/Game/GI_Ascension.GI_Ascension_C|GetEnnemis%20Rencontré%20Récemment _gi_ascension_2))
  ;[1 0 0.9844] Regarde si on a rencontré 3 ennemis ou +
  (if (>= (Utilities|Array|Length _ennemis_rencontré_récemment) 3)
    ;[1 0 0.4453] Si oui
    (Utilities|Array|RemoveIndex _ennemis_rencontré_récemment_2)
    (Utilities|Array|Add _ennemis_rencontré_récemment_2 (Variables|Default|GetEnnemiGénéré))
    (else
      ;[0.3359 0 1] Si non, rajoute l'ennemi dans la liste des ennemis rencontrés
      (Utilities|Array|Add _ennemis_rencontré_récemment (Variables|Default|GetEnnemiGénéré)))))