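; Special combat encounter actor for exploration: a named mannequin that the player approaches to set up a fight against a specific enemy.
; The construction script fills the name text from the enemy data table using the instance's enemy index.
; BeginPlay waits briefly for the main camera to settle, then turns the name toward it once.
; Sphere overlap toggles the button prompt and, on entry, passes the enemy index to the GameInstance and sets the GameMode's interaction state.
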(event OnComponentBeginOverlap(CollisionSphere)
  (params (OverlappedComponent :type Primitive%20Component%20Object%20Reference) (OtherActor :type Actor%20Object%20Reference) (OtherComp :type Primitive%20Component%20Object%20Reference) (OtherBodyIndex :type Integer) (bFromSweep :type Boolean) (SweepResult :type Hit%20Result%20Structure%20%28by%20ref%29))
  ;[1 0 0.1172] Lors Overlap Instanciation Combat, lancement Combat ou Tuto Combat
  (if (== OtherActor (Variables|Default|GetThird%20Person%20Character))
    (Development|SetHiddeninGame (Variables|Default|GetTXT%20Pour%20discuter) false false)
    ;[1 0.6328 0] Lancement du Combat
    (Variables|/Game/GI_Ascension.GI_Ascension_C|SetIndex%20Ennemi%20Actuel (Variables|Default|GetGI%20Ascension) (Variables|Default|GetIndex%20Ennemi%20Instancié))
    (Variables|/Game/GM_Exploration.GM_Exploration_C|SetENUM_Interaction_Actu (Variables|Default|GetGM%20Exploration) "NewEnumerator4")))

(event OnComponentEndOverlap(CollisionSphere)
  (params (OverlappedComponent :type Primitive%20Component%20Object%20Reference) (OtherActor :type Actor%20Object%20Reference) (OtherComp :type Primitive%20Component%20Object%20Reference) (OtherBodyIndex :type Integer))
  (if (== OtherActor (Variables|Default|GetThird%20Person%20Character))
    (Development|SetHiddeninGame (Variables|Default|GetTXT%20Pour%20discuter) true false)))

(event EventBeginPlay
  ;[0 1 1] Références
  (bind _asgi_ascension (Utilities|Casting|CastToGI_Ascension (Game|GetGameInstance)))
  (Variables|Default|SetGI%20Ascension _asgi_ascension)
  (bind _asbp_third_person_character (Utilities|Casting|CastToBP_ThirdPersonCharacter (Game|GetPlayerCharacter 0)))
  (Variables|Default|SetThird%20Person%20Character _asbp_third_person_character)
  (bind _asgm_exploration (Utilities|Casting|CastToGM_Exploration (Game|GetGameMode)))
  (Variables|Default|SetGM%20Exploration _asgm_exploration)
  ;[1 0 0.04822] DELAY pour que la CAM est le temps de changer de position
  (Utilities|FlowControl|Delay 0.1)
  ;[0 0.9382 1] Suite Références
  (bind _outactors (Actor|GetAllActorsOfClass "/Game/Camera/BP_MAIN_CAM.BP_MAIN_CAM_C"))
  (bind _output_get (Variables|Default|SetMAIN%20CAM (Utilities|Array|Get(acopy) _outactors)))
  ;[1 0 0.3047] Set Text Face MAIN CAM
  (Transformation|SetWorldRotation (Variables|Default|GetNom%20Mannequin) (Math|Rotator|FindLookatRotation (Transformation|GetWorldLocation (Variables|Default|GetNom%20Mannequin)) (Transformation|GetActorLocation _output_get)) false false))

(fn ConstructionScript
  ;[0.9688 1 0] Set le nom du mannequin
  (bind _returnvalue (Utilities|GetDataTableRow "/Game/Combat/Systeme/DD_Ennemis.DD_Ennemis" (Utilities|String|StringToName (Utilities|String|ToString(Integer) (Variables|Default|GetIndex%20Ennemi%20Instancié))))
    (:then
      (Rendering|Components|TextRender|SetText (Variables|Default|GetNom%20Mannequin) (.Nom (Utilities|Struct|BreakSTRUCT_Ennemis _returnvalue))))))